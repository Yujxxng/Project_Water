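; Switch actor that slides the Cube component of a referenced Door when interacted with.
; Interact toggles IsComplete and prints on or off; only the on branch advances a FlipFlop that alternately plays and reverses a Timeline, so the door changes direction on every other interaction.
; The Timeline's DoorTrack drives a relative-location lerp that raises the cube vertically from its local origin.
; An unconnected world-location variant remains in the graph.
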(event `self.Interact`
  (if (not (`self.isComplete?`))
    (set `self.isComplete?` true)
    (`KismetSystemLibrary.PrintString` "on")
    (`/Engine/EditorBlueprintResources/StandardMacros.FlipFlop`
      (:`A`
        (bind (_direction _door_track) (`Timeline|Timeline` :!label _label)
          (:`Update`
            (`|ExecutionSequence`
              (:`then_0`
                (`SceneComponent.K2_SetRelativeLocation` (`/Game/Actor/BP_SlidingDoor.Cube` (`self.Door`)) (`KismetMathLibrary.VLerp` (0.0 0.0 0.0) (0.0 0.0 100.0) _door_track) false false))))))
      (:`B`
        (goto _label :!via `Reverse`)))
    (else
      (set `self.isComplete?` false)
      (`KismetSystemLibrary.PrintString` "off"))))

(fn `UserConstructionScript`)