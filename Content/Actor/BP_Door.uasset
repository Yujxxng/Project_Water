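; BP_Door is a key-locked double door that swings open and closed on interaction.
; PickUpKey sets a HasKey flag, and Interact does nothing until that flag is set.
; A FlipFlop alternates between playing and reversing a Timeline, whose track drives a Lerp on each leaf's yaw so Left and Right rotate in opposite directions.
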(event `/Game/Actor/BPI_Interact.Interact`
  (if (`self.Has Key?`)
    (`/Engine/EditorBlueprintResources/StandardMacros.FlipFlop`
      (:`A`
        (bind (_direction _door_track) (`Timeline|Timeline` :!label _label)
          (:`Update`
            (`|ExecutionSequence`
              (:`then_0`
                (`SceneComponent.K2_SetRelativeRotation` (`self.Left`) (`KismetMathLibrary.MakeRotator` 0.0 0.0 (`KismetMathLibrary.Lerp` 0.0 -70.0 _door_track)) false false))
              (:`then_1`
                (`SceneComponent.K2_SetRelativeRotation` (`self.Right`) (`KismetMathLibrary.MakeRotator` 0.0 0.0 (`KismetMathLibrary.Lerp` 0.0 70.0 _door_track)) false false))))))
      (:`B`
        (goto _label :!via `Reverse`)))))

(event `/Game/Actor/BPI_Door.Pick Up Key`
  (set `self.Has Key?` true))

(fn `UserConstructionScript`)