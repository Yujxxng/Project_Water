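; Signal emitter actor that sends on and off signals to its linked receivers, optionally with a camera cutaway to show them.
; BeginPlay offsets the camera point to world space and, if no focus point is set, averages receiver locations.
; Attention-flagged signals hand the points and emitter to MyPlayerController's second camera instead of signalling directly.
; Signalling receivers starts a blend-duration timer, which resets the camera only if OnAttention is set.
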(event `self.ReceiveBeginPlay`
  (`self.InitializeEmitter`))

(event `CompleteActivationReceivers`
  (if (`self.bOnAttention`)
    (bind _asmy_player_controller (cast `/Game/Player/MyPlayerController` (`GameplayStatics.GetPlayerController` 0)))
    (`/Game/Player/MyPlayerController.ResetCamera` _asmy_player_controller)))

(fn `ActiveReceivers`
  (for _array_element (`self.Receivers`)
    (`/Game/Actor/InteractActors/BPI_Signal.SendOnSignal` _array_element))
  (bind _asmy_player_controller (cast `/Game/Player/MyPlayerController` (`GameplayStatics.GetPlayerController` 0)))
  (`KismetSystemLibrary.K2_SetTimer` null "CompleteActivationReceivers" (`/Game/Player/MyPlayerController.BlendDuration` _asmy_player_controller)))

(fn `CallSetSecondCamera`
  (params (bActive :type Boolean))
  (bind _asmy_player_controller (cast `/Game/Player/MyPlayerController` (`GameplayStatics.GetPlayerController` 0)))
  (`/Game/Player/MyPlayerController.SetSecondCamera` _asmy_player_controller (`self.CameraLocation`) (`self.AttentionLocation`) self bActive))

(fn `EmitOffSignal`
  (if (`self.bOffAttention`)
    (`self.CallSetSecondCamera` false)
    (else
      (`self.InactiveReceivers`))))

(fn `EmitOnSignal`
  (if (`self.bOnAttention`)
    (`self.CallSetSecondCamera` true)
    (else
      (`self.ActiveReceivers`))))

(fn `InactiveReceivers`
  (for _array_element (`self.Receivers`)
    (`/Game/Actor/InteractActors/BPI_Signal.SendOffSignal` _array_element))
  (bind _asmy_player_controller (cast `/Game/Player/MyPlayerController` (`GameplayStatics.GetPlayerController` 0)))
  (`KismetSystemLibrary.K2_SetTimer` null "CompleteActivationReceivers" (`/Game/Player/MyPlayerController.BlendDuration` _asmy_player_controller)))

(fn `InitializeEmitter`
  (bind _returnvalue (`self.K2_GetActorLocation`))
  (bind _attentionlocation (`self.AttentionLocation`))
  (bind _receivers (`self.Receivers`))
  (if (or (`self.bOnAttention`) (`self.bOffAttention`))
    ;[1 1 1] Local to World
    (set `self.CameraLocation` (+ (`self.CameraLocation`) _returnvalue))
    (if (`KismetMathLibrary.Vector_IsZero` (`self.AttentionLocation`))
      (for _array_element _receivers
        (set `self.AttentionLocation` (+ (`self.K2_GetActorLocation` _array_element) _attentionlocation)))
      (set `self.AttentionLocation` (/ _attentionlocation (`KismetArrayLibrary.Array_Length` _receivers)))
      (else
        (set `self.AttentionLocation` (+ (`self.AttentionLocation`) _returnvalue))))))

(fn `UserConstructionScript`)