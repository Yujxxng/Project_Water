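; BP_Platform_Moving is an interactable platform actor that moves along a Destination offset from its starting location.
; At BeginPlay it scales the offset by actor scale, then the MovementGraph timeline drives the position along that vector at Speed.
; Tick plays the timeline while unfrozen; when frozen it stops it, or restarts it from the initial location every frame if StartBegin is set.
; Activate and Inactivate both simply toggle Freeze.
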(event `self.ReceiveBeginPlay`
  (bind _destination (`self.Destination`))
  (set `self.InitialLocation` (`self.K2_GetActorLocation`))
  (set `self.Destination` (* (`self.Destination`) (`self.GetActorScale3D`)))
  (set `self.ForwardVector` (`KismetMathLibrary.Normal` _destination))
  (set `self.Distance` (`KismetMathLibrary.VSize` _destination)))

(event `self.ReceiveTick`
  (params (DeltaSeconds :type "Float (single-precision)"))
  (`TimelineComponent.SetPlayRate` (`self.MovementGraph`) (`self.Speed`))
  (if (`self.Freeze`)
    (if (`self.bStartBegin`)
      (`self.K2_SetActorLocation` (`self.InitialLocation`))
      (bind (_direction _movementvalue) (`Timeline|MovementGraph` :!via `PlayFromStart` :!label _label)
        (:`Update`
          (`self.K2_SetActorLocation` (+ (* (* _movementvalue (`self.Distance`)) (`self.ForwardVector`)) (`self.InitialLocation`)))))
      (else
        (goto _label :!via `Stop`)))
    (else
      (goto _label))))

(fn `Activate`
  (set `self.Freeze` (not (`self.Freeze`))))

(fn `Inactivate`
  (set `self.Freeze` (not (`self.Freeze`))))

(fn `UserConstructionScript`
  (`parent.UserConstructionScript`))