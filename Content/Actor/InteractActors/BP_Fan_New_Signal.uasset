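; Switchable fan actor whose wind pushes the player character along its arrow direction while in Vapor state.
; Construction script sizes the capsule trigger and wind speed from Height.
; Tick applies an impulse near the fan, then cosine-falloff acceleration with random jitter, damping lateral velocity once locked onto the axis.
; Vertical fans cap speed and damp near the top; activation toggles drive blade material spin and wind particles.
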(event `self.ReceiveBeginPlay`
  (bind _returnvalue (`GameplayStatics.GetPlayerCharacter` 0))
  (bind _horizontalforcemultiplier (`self.HorizontalForceMultiplier`))
  (bind _height (`self.Height`))
  (bind (_direction_x _direction_y _direction_z) (`KismetMathLibrary.BreakVector` (`self.Direction`)))
  (set `self.Direction` (`KismetMathLibrary.GetForwardVector` (`SceneComponent.K2_GetComponentRotation` (`self.Arrow`))))
  (set `self.PlayerMovement_0` (`Character.CharacterMovement` _returnvalue))
  (bind _asproject_water_character (cast `ProjectWaterCharacter` _returnvalue))
  (set `self.PlayerState` (`ProjectWaterCharacter.CharacterState` _asproject_water_character))
  (if (< (`KismetMathLibrary.Abs` (- _direction_z 1.0)) 0.1)
    (set `self.bVertical` true)
    (bind (_outradius _outhalfheight) (`CapsuleComponent.GetScaledCapsuleSize` (`Character.CapsuleComponent` _asproject_water_character)))
    (set `self.PlayerHalfCapsuleforDirection` _outhalfheight)
    (else
      (set `self.bVertical` false)
      (set `self.PlayerHalfCapsuleforDirection` _outradius)
      (set `self.Impulse` (* (`self.Impulse`) _horizontalforcemultiplier))
      (set `self.Accerelation` (* (`self.Accerelation`) _horizontalforcemultiplier))))
  (bind _returnvalue_2 (`PrimitiveComponent.CreateDynamicMaterialInstance` (`self.Fan`) 1 "/Game/Materials/M_Fan_Inst.M_Fan_Inst" "None"))
  (set `self.MaterialInstance` _returnvalue_2)
  (set `self.RotationSpeed` (/ (`self.Height`) 400.0))
  (`self.RotateFanMaterial`)
  ;[1 1 1] Height 1000, Accerelation 15, VelocityLimit 320, ThresholdUpper30
  (set `self.Accerelation` (* _height (`self.Accerelation`) 0.001))
  (set `self.VelocityLimit` (* _height (`self.VelocityLimit`) 0.001))
  (set `self.ThresholdUpper` (* _height (`self.ThresholdUpper`) 0.001))
  (`self.SetWindEffect`))

(event `self.ReceiveActorBeginOverlap`
  (params (OtherActor :type "Actor Object Reference"))
  (set `self.bOverlapped` true))

(event `self.ReceiveActorEndOverlap`
  (params (OtherActor :type "Actor Object Reference"))
  (set `self.bOverlapped` false))

(event `self.ReceiveTick`
  (params (DeltaSeconds :type "Float (single-precision)"))
  (bind _returnvalue (`self.K2_GetActorLocation`))
  (bind _direction (`self.Direction`))
  (bind _playermovement_0 (`self.PlayerMovement_0`))
  (bind _bvertical (`self.bVertical`))
  (bind _direction_2 (`self.Direction`))
  (bind _returnvalue_2 (`self.K2_GetActorLocation` (`GameplayStatics.GetPlayerCharacter` 0)))
  (bind _velocity (`MovementComponent.Velocity` _playermovement_0))
  (bind _returnvalue_3 (- _returnvalue_2 _returnvalue))
  (bind _returnvalue_4 (* _direction_2 (`KismetMathLibrary.Dot_VectorVector` _velocity _direction_2)))
  (bind _returnvalue_5 (`KismetMathLibrary.Dot_VectorVector` (- (- _returnvalue_2 (* (`self.PlayerHalfCapsuleforDirection`) (`self.Direction`))) _returnvalue) _direction))
  (bind _returnvalue_6 (* (+ (* (`KismetMathLibrary.DegCos` (* (/ _returnvalue_5 (`self.Height`)) 90.0)) (`self.Accerelation`)) (`KismetMathLibrary.RandomFloatInRange` -5.0 7.0)) _direction_2))
  (if (`self.bActivated`)
    (if (`self.bOverlapped`)
      (if (`|EnumEquality` (`CharacterState.State` (`self.PlayerState`)) "STATE_Vapor")
        ;[1 1 1] If player close to fan for Direction, add impulse to jump
        (if (< _returnvalue_5 (`self.ThresholdUnder`))
          (`CharacterMovementComponent.AddImpulse` (`self.PlayerMovement_0`) (* (`self.Direction`) (`self.Impulse`)) false)
          (else
            ;[1 1 1] If player is lower than Height for Direction, set velocity
            (if (< _returnvalue_5 (- (`self.Height`) (`self.ThresholdUpper`)))
              (if _bvertical
                (if (<= (`KismetMathLibrary.Dot_VectorVector` _velocity (`self.Direction`)) (`self.VelocityLimit`))
                  (if (`self.bLocked`) :!label _label
                    (set `MovementComponent.Velocity` (+ (+ (* (- _velocity _returnvalue_4) (`self.LockForce`)) _returnvalue_4) _returnvalue_6) _playermovement_0 :!label _label_2)
                    (elif (< (`KismetMathLibrary.VSize` (- _returnvalue_3 (* _direction (`KismetMathLibrary.Dot_VectorVector` _returnvalue_3 _direction)))) 30.0)
                      (set `self.bLocked` true)
                      (goto _label_2)
                      (else
                        (set `MovementComponent.Velocity` (+ _velocity _returnvalue_6) _playermovement_0))))
                  (else
                    (`KismetSystemLibrary.PrintString` "over")))
                (else
                  (goto _label)))
              (elif _bvertical
                (`KismetSystemLibrary.PrintString` (`KismetStringLibrary.Conv_VectorToString` _velocity))
                (set `MovementComponent.Velocity` (- _velocity (* _direction_2 (`self.AltitudeDamping`))) _playermovement_0)))))))))

(fn `Activate`
  (set `self.bActivated` (not (`self.bActivated`)))
  (`self.RotateFanMaterial`)
  (`self.SetWindEffect`))

(fn `Inactivate`
  (set `self.bActivated` (not (`self.bActivated`)))
  (`self.RotateFanMaterial`)
  (`self.SetWindEffect`))

(fn `RotateFanMaterial`
  (locals (speed :type "Float (double-precision)"))
  (if (`self.bActivated`)
    (set `local.speed` (`self.RotationSpeed`))
    (else
      (set `local.speed` 0.0)))
  (`MaterialInstanceDynamic.SetScalarParameterValue` (`self.MaterialInstance`) "Speed" (`local.speed`)))

(fn `SetWindEffect`
  (bind _wind (`self.Wind`))
  (if (`self.bActivated`)
    (`NiagaraComponent.SetVariableFloat` _wind "SpawnRate" 90.0)
    (else
      (`NiagaraComponent.SetVariableFloat` _wind "SpawnRate" 0.0))))

(fn `UserConstructionScript`
  (locals (hemisphere :type "Float (double-precision)") (fanScaleZ :type "Float (double-precision)"))
  (bind _capsule (`self.Capsule`))
  (bind _capsule_2 (`self.Capsule`))
  (bind (_relativescale3d_x _relativescale3d_y _relativescale3d_z) (`KismetMathLibrary.BreakVector` (`SceneComponent.RelativeScale3D` (`self.Fan`))))
  (set `local.hemisphere` (- (`CapsuleComponent.GetUnscaledCapsuleHalfHeight` _capsule_2) (`CapsuleComponent.GetUnscaledCapsuleHalfHeight_WithoutHemisphere` _capsule_2)))
  (set `local.fanScaleZ` _relativescale3d_z)
  (`CapsuleComponent.SetCapsuleHalfHeight` _capsule (/ (* (+ (`self.Height`) (`local.hemisphere`)) 0.5) (`local.fanScaleZ`)) true)
  (`SceneComponent.K2_SetRelativeLocation` _capsule (`KismetMathLibrary.MakeVector` 0.0 0.0 (/ (* (- (`self.Height`) (`local.hemisphere`)) 0.5) (`local.fanScaleZ`))) false false)
  (`NiagaraComponent.SetVariableFloat` (`self.Wind`) "Speed" (* (`self.Height`) 0.01)))