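; Toggleable moving platform that starts hidden without collision and travels from its initial location along a Destination offset.
; The MovementGraph timeline, with play rate set by Speed, scales that offset to position the actor.
; Activate shows the platform and Inactivate hides it, setting collision to match and flipping Freeze.
; Tick plays the timeline unless Freeze is set, then either stops it or, with StartBegin, restarts it from the start every frame.
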(event `self.ReceiveBeginPlay`
  (bind _bvisible (`self.bVisible`))
  (bind _destination (`self.Destination`))
  (set `self.InitialLocation` (`self.K2_GetActorLocation`))
  (set `self.ForwardVector` (`KismetMathLibrary.Normal` _destination))
  (set `self.Distance` (`KismetMathLibrary.VSize` _destination))
  (`TimelineComponent.SetPlayRate` (`self.MovementGraph`) (`self.Speed`))
  (set `self.bVisible` false)
  (`SceneComponent.SetVisibility` (`self.StaticMesh`) _bvisible false)
  (`self.SetActorEnableCollision` _bvisible))

(event `self.ReceiveTick`
  (params (DeltaSeconds :type "Float (single-precision)"))
  (if (`self.Freeze`)
    (if (`self.bStartBegin`)
      (`self.K2_SetActorLocation` (`self.InitialLocation`))
      (bind (_direction _movementvalue) (`Timeline|MovementGraph` :!via `PlayFromStart` :!label _label)
        (:`Update`
          (`self.K2_SetActorLocation` (+ (* (* _movementvalue (`self.Distance`)) (`self.ForwardVector`)) (`self.InitialLocation`)))))
      (else
        (goto _label :!via `Stop`)))
    (else
      (goto _label))))

(fn `Activate`
  (bind _bvisible (`self.bVisible`))
  (set `self.Freeze` (not (`self.Freeze`)))
  (set `self.bVisible` true)
  (`SceneComponent.SetVisibility` (`self.StaticMesh`) _bvisible false)
  (`self.SetActorEnableCollision` _bvisible))

(fn `Inactivate`
  (bind _bvisible (`self.bVisible`))
  (set `self.Freeze` (not (`self.Freeze`)))
  (set `self.bVisible` false)
  (`SceneComponent.SetVisibility` (`self.StaticMesh`) _bvisible false)
  (`self.SetActorEnableCollision` _bvisible))

(fn `UserConstructionScript`
  (`parent.UserConstructionScript`))