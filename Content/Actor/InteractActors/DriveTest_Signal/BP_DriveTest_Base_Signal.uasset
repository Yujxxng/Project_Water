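; BP_DriveTest_Base_Signal is a base signal actor for a drive test that records whether its trigger box is overlapped while the signal is active.
; Start arms it and sets the ring particles to the initial color; any overlap while armed sets Pass and the pass color.
; Result destroys the actor on success, or shows the fail color and clears both flags on failure.
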(event `self.Box.OnComponentBeginOverlap`
  (params (OverlappedComponent :type "PrimitiveComponent Object Reference") (OtherActor :type "Actor Object Reference") (OtherComp :type "PrimitiveComponent Object Reference") (OtherBodyIndex :type Integer) (bFromSweep :type Boolean) (SweepResult :type "HitResult Structure (by ref)"))
  (`self.ProcessOverlap`))

(event `self.Start`
  (`NiagaraComponent.SetVariableVec3` (`self.RingParticles`) "Color" (`self.InitColor`))
  (set `self.bStarted` true))

(event `self.Result`
  (params (Res :type Boolean))
  (bind _ringparticles (`self.RingParticles`))
  (if Res
    (`NiagaraComponent.SetVariableVec3` _ringparticles "Color" (`self.PassColor`))
    (`self.K2_DestroyActor`)
    (else
      (`NiagaraComponent.SetVariableVec3` _ringparticles "Color" (`self.FailColor`))
      (set `self.bStarted` false)
      (set `self.bPass` false))))

(fn `ProcessOverlap`
  (if (`self.bStarted`)
    (set `self.bPass` true)
    (`NiagaraComponent.SetVariableVec3` (`self.RingParticles`) "Color" (`self.PassColor`))))

(fn `UserConstructionScript`)