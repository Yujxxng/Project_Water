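; BP_Lever_Bool is an interactable lever that works as a two-state switch, emitting on and off signals.
; BeginPlay tilts the Joint component to negative Angle pitch.
; Each Interact flips the activation flag, emits the matching signal and plays the RotateJoint timeline forward from start or in reverse from end.
; The timeline scales its rotation value by Angle to swing the Joint.
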(event `self.ReceiveBeginPlay`
  (`parent.ReceiveBeginPlay`)
  (`SceneComponent.K2_SetRelativeRotation` (`self.Joint`) (`KismetMathLibrary.MakeRotator` 0.0 (* (`self.Angle`) -1.0)) false false))

(event `/Game/Actor/InteractActors/BPI_Interact.Interact`
  (if (not (`self.bActivated_0`))
    (set `self.bActivated_0` true)
    (`self.EmitOnSignal`)
    (bind (_direction _rotationvalue) (`Timeline|RotateJoint` :!via `PlayFromStart` :!label _label)
      (:`Update`
        (`SceneComponent.K2_SetRelativeRotation` (`self.Joint`) (`KismetMathLibrary.MakeRotator` 0.0 (* _rotationvalue (`self.Angle`))) false false)))
    (else
      (set `self.bActivated_0` false)
      (`self.EmitOffSignal`)
      (goto _label :!via `ReverseFromEnd`))))

(fn `UserConstructionScript`
  (`parent.UserConstructionScript`))