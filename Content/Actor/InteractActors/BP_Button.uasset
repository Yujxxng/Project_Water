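; BP_Button is a pressure plate that emits a signal once an actor tagged Pressable has stayed on it long enough.
; Trigger overlaps play or reverse the PlatePressure timeline, which lerps the plate's height, unless Activated is set.
; Tick accumulates overlap time and calls EmitOnSignal once that reaches the timeline's length, with OverTime blocking repeats until the overlap ends.
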(event `self.Trigger.OnComponentBeginOverlap`
  (params (OverlappedComponent :type "PrimitiveComponent Object Reference") (OtherActor :type "Actor Object Reference") (OtherComp :type "PrimitiveComponent Object Reference") (OtherBodyIndex :type Integer) (bFromSweep :type Boolean) (SweepResult :type "HitResult Structure (by ref)"))
  (if (and (`self.ActorHasTag` OtherActor "Pressable") (not (`self.bActivated`)))
    (set `self.bOverlapped` true)
    (set `self.Timer` 0.0)
    (`TimelineComponent.PlayFromStart` (`self.Plate Pressure`))))

(event `self.Trigger.OnComponentEndOverlap`
  (params (OverlappedComponent :type "PrimitiveComponent Object Reference") (OtherActor :type "Actor Object Reference") (OtherComp :type "PrimitiveComponent Object Reference") (OtherBodyIndex :type Integer))
  (if (and (`self.ActorHasTag` OtherActor "Pressable") (not (`self.bActivated`)))
    (set `self.bOverlapped` false)
    (`TimelineComponent.Reverse` (`self.Plate Pressure`))
    (set `self.bOverTime` false)))

(event `self.ReceiveTick`
  (params (DeltaSeconds :type "Float (single-precision)"))
  (if (and (`self.bOverlapped`) (not (`self.bOverTime`)))
    (bind _output_get (set `self.Timer` (+ DeltaSeconds (`self.Timer`))))
    (if (>= _output_get (`TimelineComponent.GetTimelineLength` (`self.Plate Pressure`)))
      (`self.EmitOnSignal`)
      (set `self.bOverTime` true))))

(fn `UserConstructionScript`)