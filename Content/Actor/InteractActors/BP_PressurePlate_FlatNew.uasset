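; BP_PressurePlate_FlatNew is a pressure plate interactable that sends on and off signals when actors tagged "Pressable" enter or leave its trigger.
; Trigger overlaps maintain a count of pressing actors, so the off signal fires only when the count drops to zero or below.
; Tick emits the on signal once per press, using OverTimer as a latch that resets on release.
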(event `self.Trigger.OnComponentBeginOverlap`
  (params (OverlappedComponent :type "PrimitiveComponent Object Reference") (OtherActor :type "Actor Object Reference") (OtherComp :type "PrimitiveComponent Object Reference") (OtherBodyIndex :type Integer) (bFromSweep :type Boolean) (SweepResult :type "HitResult Structure (by ref)"))
  (if (`self.ActorHasTag` OtherActor "Pressable")
    (set `self.bOverlapped` true)
    (`/Engine/EditorBlueprintResources/StandardMacros.IncrementInt` (`self.OverlapNum`))))

(event `self.Trigger.OnComponentEndOverlap`
  (params (OverlappedComponent :type "PrimitiveComponent Object Reference") (OtherActor :type "Actor Object Reference") (OtherComp :type "PrimitiveComponent Object Reference") (OtherBodyIndex :type Integer))
  (bind _overlapnum (`self.OverlapNum`))
  (if (`self.ActorHasTag` OtherActor "Pressable")
    (`/Engine/EditorBlueprintResources/StandardMacros.DecrementInt` _overlapnum
      (:`  `
        (if (<= _overlapnum 0)
          (set `self.bOverlapped` false)
          (`self.EmitOffSignal`)
          (set `self.bOverTimer` false))))))

(event `self.ReceiveTick`
  (params (DeltaSeconds :type "Float (single-precision)"))
  (if (and (`self.bOverlapped`) (not (`self.bOverTimer`)))
    (`self.EmitOnSignal`)
    (set `self.bOverTimer` true)))

(fn `UserConstructionScript`)