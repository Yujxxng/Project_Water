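; BP_PassRing is an interactable ring that reports to its parent BP_PassRing_Manager when something overlaps its box.
; It caches the manager from its attach parent on BeginPlay.
; An overlap while CheckStart is false calls SetAllRings(true) on the manager, then registers the ring through SetRing and marks it passed.
; Once SetActivated sets CheckStart, overlaps register the ring only if it is not yet passed.
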(event `self.ReceiveBeginPlay`
  (bind _asbp_pass_ring_manager (cast `/Game/Actor/InteractActors/BP_PassRing_Manager` (`self.GetAttachParentActor`)))
  (set `self.Manager` _asbp_pass_ring_manager))

(event `self.Box.OnComponentBeginOverlap`
  (params (OverlappedComponent :type "PrimitiveComponent Object Reference") (OtherActor :type "Actor Object Reference") (OtherComp :type "PrimitiveComponent Object Reference") (OtherBodyIndex :type Integer) (bFromSweep :type Boolean) (SweepResult :type "HitResult Structure (by ref)"))
  (bind _manager (`self.Manager`))
  (if (`self.bCheckStart`)
    (if (not (`self.bPassed`))
      (`/Game/Actor/InteractActors/BP_PassRing_Manager.SetRing` _manager self :!label _label)
      (set `self.bPassed` true))
    (else
      (`/Game/Actor/InteractActors/BP_PassRing_Manager.SetAllRings` _manager true)
      (goto _label))))

(fn `SetActivated`
  (params (bActive :type Boolean))
  (set `self.bCheckStart` bActive))

(fn `UserConstructionScript`)