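; Manager ring for a pass-through ring challenge that emits a signal once it and all its attached BP_PassRing actors are passed.
; BeginPlay gathers attached rings into ChildRings and counts itself in the total.
; Its first overlap activates and recolors the children, then counts itself as passed.
; SetRing recolors a reported child ring and advances the count, with debug prints, toward EmitOnSignal.
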(event `self.ReceiveBeginPlay`
  (bind _childrings (`self.ChildRings`))
  (`parent.ReceiveBeginPlay`)
  (for _array_element (`self.GetAttachedActors` true)
    (bind _asbp_pass_ring (cast `/Game/Actor/InteractActors/BP_PassRing` _array_element))
    (`BlueprintSetLibrary.Set_Add` _childrings _asbp_pass_ring))
  (bind _output_get (set `self.MaxRingNum` (`BlueprintSetLibrary.Set_Length` _childrings)))
  (`/Engine/EditorBlueprintResources/StandardMacros.IncrementInt` _output_get))

(event `self.Box.OnComponentBeginOverlap`
  (params (OverlappedComponent :type "PrimitiveComponent Object Reference") (OtherActor :type "Actor Object Reference") (OtherComp :type "PrimitiveComponent Object Reference") (OtherBodyIndex :type Integer) (bFromSweep :type Boolean) (SweepResult :type "HitResult Structure (by ref)"))
  (if (not (`self.bPassed`))
    (set `self.bPassed` true)
    (if (not (`self.bCheckStart`))
      (`self.SetAllRings` true))
    (`NiagaraComponent.SetVariableVec3` (`self.Ring`) "Color" (`self.PassColor`))
    (`self.AddCheckRing`)))

(event `SetAllRings`
  (params (bActive :type Boolean))
  (`NiagaraComponent.SetVariableVec3` (`self.Ring`) "None" (`self.InitColor`))
  (set `self.bCheckStart` true)
  (bind _result (`BlueprintSetLibrary.Set_ToArray` (`self.ChildRings`)))
  (for _array_element _result
    (`NiagaraComponent.SetVariableVec3` (`/Game/Actor/InteractActors/BP_PassRing.Ring` _array_element) "Color" (`self.InitColor`))
    (`/Game/Actor/InteractActors/BP_PassRing.SetActivated` _array_element bActive)))

(event `SetRing`
  (params (ring :type "/Game/Actor/InteractActors/BP_PassRing Object Reference"))
  (if (`BlueprintSetLibrary.Set_Contains` (`self.ChildRings`) ring)
    (`NiagaraComponent.SetVariableVec3` (`/Game/Actor/InteractActors/BP_PassRing.Ring` ring) "Color" (`self.PassColor`))
    (`self.AddCheckRing`)))

(fn `AddCheckRing`
  (`KismetSystemLibrary.PrintString` "add check ring")
  (bind _result (`/Engine/EditorBlueprintResources/StandardMacros.IncrementInt` (`self.ActivatedRingNum`))
    (:`  `
      (if (>= _result (`self.MaxRingNum`))
        (`KismetSystemLibrary.PrintString` "PASS!!!")
        (`self.EmitOnSignal`)
        (else
          (`KismetSystemLibrary.PrintString` (`KismetStringLibrary.Conv_IntToString` _result)))))))

(fn `UserConstructionScript`)