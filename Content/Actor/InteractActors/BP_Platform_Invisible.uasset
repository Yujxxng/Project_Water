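; BP_Platform_Invisible is an interactable platform that switches between visible and solid, and hidden and non-colliding.
; Activate and Inactivate both flip the Visible flag rather than setting it, so the starting value decides which state each call produces.
; Tick applies the flag every frame to the static mesh's visibility, without propagating to children, and to the whole actor's collision.
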(event `self.ReceiveTick`
  (params (DeltaSeconds :type "Float (single-precision)"))
  (bind _bvisible (`self.bVisible`))
  (`SceneComponent.SetVisibility` (`self.StaticMesh`) _bvisible false)
  (`self.SetActorEnableCollision` _bvisible))

(fn `Activate`
  (set `self.bVisible` (not (`self.bVisible`))))

(fn `Inactivate`
  (set `self.bVisible` (not (`self.bVisible`))))

(fn `UserConstructionScript`
  (`parent.UserConstructionScript`))