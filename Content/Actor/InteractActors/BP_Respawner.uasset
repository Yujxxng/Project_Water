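; BP_Respawner is an interactable actor that spawns an actor of a configurable class and can return it to the spawn point.
; On BeginPlay it spawns ActorClass at its own location and rotation with unit scale and stores the reference.
; Activate calls Respawn, which teleports that same stored actor back to the respawner's transform rather than destroying it or spawning a new one.
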(event `self.ReceiveBeginPlay`
  (bind _returnvalue (`|SpawnActorFromClass` (`self.ActorClass`) (`KismetMathLibrary.MakeTransform` (`self.K2_GetActorLocation`) (`self.K2_GetActorRotation`)) "Undefined" "MultiplyWithRoot" null null))
  (set `self.Actor` _returnvalue))

(event `Respawn`
  (`self.K2_SetActorLocationAndRotation` (`self.Actor`) (`self.K2_GetActorLocation`) (`self.K2_GetActorRotation`) false false))

(fn `Activate`
  (`self.Respawn`))

(fn `UserConstructionScript`
  (`parent.UserConstructionScript`))