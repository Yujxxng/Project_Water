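; BP_Platform_Move is an interactable platform that moves along a straight offset from its starting location, set by its Destination vector.
; A timeline scales that offset to set the actor's location without sweeping.
; Tick updates the timeline's play rate from Speed and plays or stops it according to Freeze.
; Activate and Inactivate both toggle Freeze rather than setting fixed states.
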(event `self.ReceiveBeginPlay`
  (bind _destination (`self.Destination`))
  (set `self.InitialLocation` (`self.K2_GetActorLocation`))
  (set `self.ForwardVector` (`KismetMathLibrary.Normal` _destination))
  (set `self.Distance` (`KismetMathLibrary.VSize` _destination)))

(event `self.ReceiveTick`
  (params (DeltaSeconds :type "Float (single-precision)"))
  (`TimelineComponent.SetPlayRate` (`self.MovementGraph`) (`self.Speed`))
  (if (`self.Freeze`)
    (bind (_direction _movementvalue) (`Timeline|MovementGraph` :!via `Stop` :!label _label)
      (:`Update`
        (`self.K2_SetActorLocation` (+ (* (* _movementvalue (`self.Distance`)) (`self.ForwardVector`)) (`self.InitialLocation`)))))
    (else
      (goto _label))))

(fn `Activate`
  (set `self.Freeze` (not (`self.Freeze`))))

(fn `Inactivate`
  (set `self.Freeze` (not (`self.Freeze`))))

(fn `UserConstructionScript`
  (`parent.UserConstructionScript`))