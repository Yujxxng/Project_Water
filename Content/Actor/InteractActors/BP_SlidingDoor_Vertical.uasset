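; Vertical sliding door actor in the interactable set that opens and closes when activated or inactivated.
; Activate and Inactivate call OpenDoor and CloseDoor, which play or reverse the MovementDoor timeline, whose height track sets the Door's relative Z location.
; The construction script scales the Wall mesh from the Height variable, less a fixed offset.
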(event `OpenDoor`
  (`TimelineComponent.Play` (`self.MovementDoor`)))

(event `CloseDoor`
  (`TimelineComponent.Reverse` (`self.MovementDoor`)))

(fn `Activate`
  (`self.OpenDoor`))

(fn `Inactivate`
  (`self.CloseDoor`))

(fn `UserConstructionScript`
  (`parent.UserConstructionScript`)
  (`SceneComponent.SetRelativeScale3D` (`self.Wall`) (`KismetMathLibrary.MakeVector` 3.0 0.3 (* (- (`self.Height`) 270.0) 0.01))))