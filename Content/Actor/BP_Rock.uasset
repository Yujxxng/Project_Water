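; BP_Rock is a rock the third-person character can push or pull along one axis.
; Overlapping its Forward component toggles the character's CanInteractBox flag.
; While interacting, Tick reads the character's Forward value and calls Speed/Direction, which interpolates the Rock component along its right vector without sweeping.
; Sideways input is unused, and debug prints remain throughout.
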(event `self.ReceiveBeginPlay`
  (bind _returnvalue (`GameplayStatics.GetActorOfClass` "/Game/ThirdPerson/Blueprints/BP_ThirdPersonCharacter_YJ.BP_ThirdPersonCharacter_YJ_C"))
  (set `self.CharacterRef` _returnvalue))

(event `self.ReceiveTick`
  (params (DeltaSeconds :type "Float (single-precision)"))
  (bind _characterref (`self.CharacterRef`))
  (bind _forward (`/Game/ThirdPerson/Blueprints/BP_ThirdPersonCharacter_YJ.Forward` (`self.CharacterRef`)))
  (if (`/Game/ThirdPerson/Blueprints/BP_ThirdPersonCharacter_YJ.IsInteractingBox?` _characterref)
    (if (`/Game/ThirdPerson/Blueprints/BP_ThirdPersonCharacter_YJ.CanInteractBox?` _characterref)
      (`|ExecutionSequence`
        (:`then_0`
          (if (== _forward 0.0)
            (`KismetSystemLibrary.PrintString` "Not Moving F/B")
            (elif (>= _forward 0.1)
              (`KismetSystemLibrary.PrintString` "Moving F")
              (`self.Speed/Direction` true -34.0)
              (else
                (`KismetSystemLibrary.PrintString` "Moving B")
                (`self.Speed/Direction` true 34.0)))))))))

(event `self.Forward.OnComponentBeginOverlap`
  (params (OverlappedComponent :type "PrimitiveComponent Object Reference") (OtherActor :type "Actor Object Reference") (OtherComp :type "PrimitiveComponent Object Reference") (OtherBodyIndex :type Integer) (bFromSweep :type Boolean) (SweepResult :type "HitResult Structure (by ref)"))
  (`KismetSystemLibrary.PrintString` "Can Interact")
  (set `/Game/ThirdPerson/Blueprints/BP_ThirdPersonCharacter_YJ.CanInteractBox?` true (`self.CharacterRef`)))

(event `self.Forward.OnComponentEndOverlap`
  (params (OverlappedComponent :type "PrimitiveComponent Object Reference") (OtherActor :type "Actor Object Reference") (OtherComp :type "PrimitiveComponent Object Reference") (OtherBodyIndex :type Integer))
  (`KismetSystemLibrary.PrintString` "Cant Interact")
  (set `/Game/ThirdPerson/Blueprints/BP_ThirdPersonCharacter_YJ.CanInteractBox?` false (`self.CharacterRef`)))

(fn `UserConstructionScript`)