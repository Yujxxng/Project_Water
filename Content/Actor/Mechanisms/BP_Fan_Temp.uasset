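; Fan mechanism that pushes the third-person player character along its Arrow direction, like an updraft.
; Each tick a debug-drawn capsule trace reaches MaxHeight from Base, adding force scaled by a cosine falloff on hit world Z.
; Capsule overlap records each character's gravity scale and restores it on exit, though nothing here alters it.
; Sphere-trace and LaunchCharacter alternatives remain unconnected.
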(event `self.ReceiveTick`
  (params (DeltaSeconds :type "Float (single-precision)"))
  (bind _returnvalue (`SceneComponent.K2_GetComponentLocation` (`self.Base`)))
  (bind _returnvalue_2 (`KismetMathLibrary.GetForwardVector` (`SceneComponent.K2_GetComponentRotation` (`self.Arrow`))))
  (bind (_outhits _returnvalue_3) (`KismetSystemLibrary.CapsuleTraceMultiForObjects` :`Start` _returnvalue :`End` (+ _returnvalue (* _returnvalue_2 (`self.MaxHeight`))) :`ObjectTypes` (`|MakeArray` "ObjectTypeQuery3" :!type "EObjectTypeQuery Enum") :`DrawDebugType` "ForOneFrame"))
  (if _returnvalue_3
    (for _array_element _outhits
      (bind (_bblockinghit _binitialoverlap _time _distance _location _impactpoint _normal _impactnormal _physmat _hitactor) (`GameplayStatics.BreakHitResult` _array_element))
      (bind _asbp_third_person_character_yj (cast `/Game/ThirdPerson/Blueprints/BP_ThirdPersonCharacter_YJ` _hitactor)
        (:`then`
          (`CharacterMovementComponent.AddForce` (`Character.CharacterMovement` _asbp_third_person_character_yj) (* (/ (`KismetMathLibrary.DegCos` (* (/ (.z _location) (`self.MaxHeight`)) 90.0)) 2.0) (* _returnvalue_2 130.0))))
        (:`CastFailed`
          (`KismetSystemLibrary.PrintString` "cast failed"))))))

(event `self.Capsule.OnComponentBeginOverlap`
  (params (OverlappedComponent :type "PrimitiveComponent Object Reference") (OtherActor :type "Actor Object Reference") (OtherComp :type "PrimitiveComponent Object Reference") (OtherBodyIndex :type Integer) (bFromSweep :type Boolean) (SweepResult :type "HitResult Structure (by ref)"))
  (bind `_as캐릭터` (cast `Character` OtherActor))
  (`BlueprintMapLibrary.Map_Add` (`self.Overlapped`) OtherActor (`CharacterMovementComponent.GravityScale` (`Character.CharacterMovement` `_as캐릭터`))))

(event `self.Capsule.OnComponentEndOverlap`
  (params (OverlappedComponent :type "PrimitiveComponent Object Reference") (OtherActor :type "Actor Object Reference") (OtherComp :type "PrimitiveComponent Object Reference") (OtherBodyIndex :type Integer))
  (bind `_as캐릭터` (cast `Character` OtherActor))
  (set `CharacterMovementComponent.GravityScale` (`BlueprintMapLibrary.Map_Find` (`self.Overlapped`) `_as캐릭터`) (`Character.CharacterMovement` `_as캐릭터`)))

(fn `UserConstructionScript`)