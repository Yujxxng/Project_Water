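; BP_DriveTest_Start is the start trigger of a drive test, coordinating a set of course actors.
; Overlapping its Box starts every entry in Courses, then calls its own Start and ProcessOverlap.
; The End event clears Success if any course has not passed, then sends that overall result to each course and to itself through Result.
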(event `self.Box.OnComponentBeginOverlap`
  (params (OverlappedComponent :type "PrimitiveComponent Object Reference") (OtherActor :type "Actor Object Reference") (OtherComp :type "PrimitiveComponent Object Reference") (OtherBodyIndex :type Integer) (bFromSweep :type Boolean) (SweepResult :type "HitResult Structure (by ref)"))
  (for _array_element (`self.Courses`)
    (`self.Start` _array_element))
  (`/Game/Actor/Mechanisms/DriveTest/BPI_DriveTest.Start`)
  (`self.ProcessOverlap`))

(event `/Game/Actor/Mechanisms/DriveTest/BPI_DriveTest.End`
  (bind _bsuccess (`self.bSuccess`))
  (bind _courses (`self.Courses`))
  (for _array_element _courses
    (if (not (`/Game/Actor/Mechanisms/DriveTest/BP_DriveTest_Base.bPass` _array_element))
      (set `self.bSuccess` false)))
  (for _array_element_2 _courses
    (`/Game/Actor/Mechanisms/DriveTest/BPI_DriveTest.Result` _array_element_2 _bsuccess))
  (`/Game/Actor/Mechanisms/DriveTest/BPI_DriveTest.Result` _bsuccess))

(fn `UserConstructionScript`
  (`parent.UserConstructionScript`))