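; Spring pad actor that launches a Character hitting it fast enough against its arrow direction, scaling the launch with incoming speed.
; Capsule overlap checks velocity along that direction, then launches and disarms the pad; the next Character overlap while disarmed re-arms it without launching.
; A dynamic plate material shows state and impact strength, with Tick running a color-blend timeline while armed.
; Impact speeds are printed for debugging.
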(event `self.ReceiveBeginPlay`
  (bind _returnvalue (`PrimitiveComponent.CreateDynamicMaterialInstance` (`self.Plate`) 0 "/Game/Materials/MI_OnOff.MI_OnOff" "None"))
  (bind _output_get (set `self.MaterialInstance` _returnvalue))
  (`MaterialInstanceDynamic.SetVectorParameterValue` _output_get "Color" (`self.ActiveColor`))
  (set `self.Direction` (`KismetMathLibrary.GetForwardVector` (`SceneComponent.K2_GetComponentRotation` (`self.Arrow`)))))

(event `self.Capsule.OnComponentBeginOverlap`
  (params (OverlappedComponent :type "PrimitiveComponent Object Reference") (OtherActor :type "Actor Object Reference") (OtherComp :type "PrimitiveComponent Object Reference") (OtherBodyIndex :type Integer) (bFromSweep :type Boolean) (SweepResult :type "HitResult Structure (by ref)"))
  (bind _returnvalue (`self.GetVelocity` OtherActor))
  (bind _materialinstance (`self.MaterialInstance`))
  (bind _returnvalue_2 (* (`KismetMathLibrary.Dot_VectorVector` _returnvalue (`self.Direction`)) -1.0))
  (bind `_as캐릭터` (cast `Character` OtherActor))
  (if (`self.bActivated`)
    (if (>= _returnvalue_2 (`self.TriggerSpeed`))
      (`KismetSystemLibrary.PrintString` (`KismetStringLibrary.Conv_DoubleToString` _returnvalue_2))
      (`Character.LaunchCharacter` `_as캐릭터` (* (* (`KismetMathLibrary.VSize` _returnvalue) (`self.LaunchMultiplier`)) (`self.Direction`)) true true)
      (set `self.bActivated` false)
      (`MaterialInstanceDynamic.SetVectorParameterValue` _materialinstance "Color" (`KismetMathLibrary.LinearColorLerp` (`self.MinColor`) (`self.MaxColor`) (/ _returnvalue_2 1300.0))))
    (else
      (set `self.bActivated` true)
      (`MaterialInstanceDynamic.SetVectorParameterValue` _materialinstance "Color" (`self.ActiveColor`)))))

(event `self.Plate.OnComponentHit`
  (params (HitComponent :type "PrimitiveComponent Object Reference") (OtherActor :type "Actor Object Reference") (OtherComp :type "PrimitiveComponent Object Reference") (NormalImpulse :type "Vector Structure") (Hit :type "HitResult Structure (by ref)"))
  (`KismetSystemLibrary.PrintString` (`KismetStringLibrary.Conv_DoubleToString` (`KismetMathLibrary.VSize` (`self.GetVelocity` OtherActor)))))

(event `self.ReceiveTick`
  (params (DeltaSeconds :type "Float (single-precision)"))
  (if (`self.bActivated`)
    (bind (_direction _alpha) (`Timeline|ChangeColor` :!label _label)
      (:`Update`
        (`MaterialInstanceDynamic.SetVectorParameterValue` (`self.MaterialInstance`) "Color" (`KismetMathLibrary.LinearColorLerp` (`self.MinColor`) (`self.MaxColor`) _alpha))))
    (else
      (goto _label :!via `Stop`))))

(fn `UserConstructionScript`)