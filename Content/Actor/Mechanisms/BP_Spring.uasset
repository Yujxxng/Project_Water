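; BP_Spring is a spring mechanism that launches characters straight up when they land on it fast enough.
; On box overlap while active, it checks downward speed against a threshold, then overrides velocity with an upward launch scaled from impact speed.
; Launching deactivates the spring and recolors its plate through a dynamic material instance.
; The next overlap by any actor only re-arms it and restores the initial color.
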(event `self.ReceiveBeginPlay`
  (bind _returnvalue (`PrimitiveComponent.CreateDynamicMaterialInstance` (`self.Plate`) 0 "/Game/Materials/MI_OnOff.MI_OnOff" "None"))
  (bind _output_get (set `self.MaterialInstance` _returnvalue))
  (bind _returnvalue_2 (`MaterialInstanceDynamic.K2_GetVectorParameterValue` _output_get "Color"))
  (set `self.InitialColor` (`KismetMathLibrary.Conv_LinearColorToVector` _returnvalue_2)))

(event `self.Box.OnComponentBeginOverlap`
  (params (OverlappedComponent :type "PrimitiveComponent Object Reference") (OtherActor :type "Actor Object Reference") (OtherComp :type "PrimitiveComponent Object Reference") (OtherBodyIndex :type Integer) (bFromSweep :type Boolean) (SweepResult :type "HitResult Structure (by ref)"))
  (bind _returnvalue (`self.GetVelocity` OtherActor))
  (bind _materialinstance (`self.MaterialInstance`))
  (if (`self.bActivated`)
    (bind `_as캐릭터` (cast `Character` OtherActor))
    (if (>= (* (.z _returnvalue) -1.0) (`self.TriggerZSpeed`))
      (`Character.LaunchCharacter` `_as캐릭터` (`KismetMathLibrary.MakeVector` 0.0 0.0 (* (`KismetMathLibrary.VSize` _returnvalue) (`self.Multiplier`))) true true)
      (set `self.bActivated` false)
      (`MaterialInstanceDynamic.SetVectorParameterValue` _materialinstance "Color" (`KismetMathLibrary.Conv_VectorToLinearColor` (`self.InactiveColor`))))
    (else
      (set `self.bActivated` true)
      (`MaterialInstanceDynamic.SetVectorParameterValue` _materialinstance "Color" (`KismetMathLibrary.Conv_VectorToLinearColor` (`self.InitialColor`))))))

(fn `UserConstructionScript`)