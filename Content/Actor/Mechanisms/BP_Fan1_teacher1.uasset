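; BP_Fan1_teacher1 is a fan mechanism that pushes overlapping characters along its Arrow to lift or hover them.
; The trigger stores each Character's gravity scale on entry and restores it on exit.
; Each tick, BP_ThirdPersonCharacter_YJ actors below half MaxHeight in world Z receive an impulse.
; At or above that height, nearly stationary ones get near-zero gravity so they float.
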(event `self.ReceiveTick`
  (params (DeltaSeconds :type "Float (single-precision)"))
  (bind _keys (`BlueprintMapLibrary.Map_Keys` (`self.Overlapped`)))
  (for _array_element _keys
    (bind _asbp_third_person_character_yj (cast `/Game/ThirdPerson/Blueprints/BP_ThirdPersonCharacter_YJ` _array_element))
    (bind (_returnvalue_x _returnvalue_y _returnvalue_z) (`KismetMathLibrary.BreakVector` (`self.K2_GetActorLocation` _asbp_third_person_character_yj)))
    (if (>= _returnvalue_z (* (`self.MaxHeight`) 0.5))
      (bind _charactermovement (`Character.CharacterMovement` _asbp_third_person_character_yj))
      (if (<= (`KismetMathLibrary.VSize` (`self.GetVelocity` (`PawnMovementComponent.GetPawnOwner` _charactermovement))) 3.0)
        (set `CharacterMovementComponent.GravityScale` 0.01 _charactermovement))
      (else
        (`CharacterMovementComponent.AddImpulse` _charactermovement (* (`KismetMathLibrary.GetForwardVector` (`SceneComponent.K2_GetComponentRotation` (`self.Arrow`))) (`KismetMathLibrary.RandomFloatInRange` 6.0 6.0)) false)))))

(event `self.Trigger.OnComponentBeginOverlap`
  (params (OverlappedComponent :type "PrimitiveComponent Object Reference") (OtherActor :type "Actor Object Reference") (OtherComp :type "PrimitiveComponent Object Reference") (OtherBodyIndex :type Integer) (bFromSweep :type Boolean) (SweepResult :type "HitResult Structure (by ref)"))
  (bind `_as캐릭터` (cast `Character` OtherActor))
  (bind _gravityscale (`CharacterMovementComponent.GravityScale` (`Character.CharacterMovement` `_as캐릭터`)))
  (`BlueprintMapLibrary.Map_Add` (`self.Overlapped`) OtherActor _gravityscale)
  (`KismetSystemLibrary.PrintString` (`KismetStringLibrary.Conv_DoubleToString` _gravityscale)))

(event `self.Trigger.OnComponentEndOverlap`
  (params (OverlappedComponent :type "PrimitiveComponent Object Reference") (OtherActor :type "Actor Object Reference") (OtherComp :type "PrimitiveComponent Object Reference") (OtherBodyIndex :type Integer))
  (bind _overlapped (`self.Overlapped`))
  (bind `_as캐릭터` (cast `Character` OtherActor))
  (bind _value (`BlueprintMapLibrary.Map_Find` _overlapped `_as캐릭터`))
  (bind _output_get (set `CharacterMovementComponent.GravityScale` _value (`Character.CharacterMovement` `_as캐릭터`)))
  (`KismetSystemLibrary.PrintString` (`KismetStringLibrary.Conv_DoubleToString` _value))
  (`BlueprintMapLibrary.Map_Remove` _overlapped OtherActor))

(fn `UserConstructionScript`)