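; Fan mechanism that pushes the player character along its arrow direction while the character overlaps it in Vapor state.
; Height sizes the capsule in the construction script and scales material speed and force tuning at BeginPlay.
; Tick applies an impulse near the fan, then cosine-falloff acceleration with random jitter up to the height threshold.
; Vertical fans add a velocity cap and altitude damping; horizontal fans use a force multiplier.
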(event `self.ReceiveBeginPlay`
  (bind _returnvalue (`GameplayStatics.GetPlayerCharacter` 0))
  (bind _horizontalforcemultiplier (`self.HorizontalForceMultiplier`))
  (bind _height (`self.Height`))
  (bind (_direction_x _direction_y _direction_z) (`KismetMathLibrary.BreakVector` (`self.Direction`)))
  (set `self.Direction` (`KismetMathLibrary.GetForwardVector` (`SceneComponent.K2_GetComponentRotation` (`self.Arrow`))))
  (set `self.PlayerMovement` (`Character.CharacterMovement` _returnvalue))
  (bind _asproject_water_character (cast `ProjectWaterCharacter` _returnvalue))
  (set `self.PlayerState` (`ProjectWaterCharacter.CharacterState` _asproject_water_character))
  (if (< (`KismetMathLibrary.Abs` (- _direction_z 1.0)) 0.1)
    (set `self.bVertical` true)
    (bind (_outradius _outhalfheight) (`CapsuleComponent.GetScaledCapsuleSize` (`Character.CapsuleComponent` _asproject_water_character)))
    (set `self.PlayerHalfCapsuleforDirection` _outhalfheight)
    (else
      (set `self.bVertical` false)
      (set `self.PlayerHalfCapsuleforDirection` _outradius)
      (set `self.Impulse` (* (`self.Impulse`) _horizontalforcemultiplier))
      (set `self.Accerelation` (* (`self.Accerelation`) _horizontalforcemultiplier))))
  (bind _returnvalue_2 (`PrimitiveComponent.CreateDynamicMaterialInstance` (`self.Fan`) 1 "/Game/Materials/M_Fan_Inst.M_Fan_Inst" "None"))
  (`MaterialInstanceDynamic.SetScalarParameterValue` _returnvalue_2 "Speed" (/ (`self.Height`) 400.0))
  ;[1 1 1] Height 1000, Accerelation 15, VelocityLimit 320, ThresholdUpper30
  (set `self.Accerelation` (* _height (`self.Accerelation`) 0.001))
  (set `self.VelocityLimit` (* _height (`self.VelocityLimit`) 0.001))
  (set `self.ThresholdUpper` (* _height (`self.ThresholdUpper`) 0.001)))

(event `self.ReceiveActorBeginOverlap`
  (params (OtherActor :type "Actor Object Reference"))
  (set `self.bOverlapped` true))

(event `self.ReceiveActorEndOverlap`
  (params (OtherActor :type "Actor Object Reference"))
  (set `self.bOverlapped` false))

(event `self.ReceiveTick`
  (params (DeltaSeconds :type "Float (single-precision)"))
  (bind _playermovement (`self.PlayerMovement`))
  (bind _bvertical (`self.bVertical`))
  (bind _direction (`self.Direction`))
  (bind _velocity (`MovementComponent.Velocity` _playermovement))
  (bind _returnvalue (`KismetMathLibrary.Dot_VectorVector` (- (- (`self.K2_GetActorLocation` (`GameplayStatics.GetPlayerCharacter` 0)) (* (`self.PlayerHalfCapsuleforDirection`) (`self.Direction`))) (`self.K2_GetActorLocation`)) (`self.Direction`)))
  (if (`self.bOverlapped`)
    (if (`|EnumEquality` (`CharacterState.State` (`self.PlayerState`)) "STATE_Vapor")
      ;[1 1 1] If player close to fan for Direction, add impulse to jump
      (if (< _returnvalue (`self.ThresholdUnder`))
        (`CharacterMovementComponent.AddImpulse` (`self.PlayerMovement`) (* (`self.Direction`) (`self.Impulse`)) false)
        (else
          ;[1 1 1] If player is lower than Height for Direction, set velocity
          (if (< _returnvalue (- (`self.Height`) (`self.ThresholdUpper`)))
            (if _bvertical
              (if (<= (`KismetMathLibrary.Dot_VectorVector` _velocity (`self.Direction`)) (`self.VelocityLimit`))
                (set `MovementComponent.Velocity` (+ _velocity (* (+ (* (`KismetMathLibrary.DegCos` (* (/ _returnvalue (`self.Height`)) 90.0)) (`self.Accerelation`)) (`KismetMathLibrary.RandomFloatInRange` -5.0 7.0)) _direction)) _playermovement :!label _label) ; lock 적용 안하는 노드!!!!!!!!!
                (else
                  (`KismetSystemLibrary.PrintString` "nnnnnn")))
              (else
                (goto _label)))
            (elif _bvertical
              (set `MovementComponent.Velocity` (- _velocity (* _direction (`self.AltitudeDamping`))) _playermovement))))))))

(fn `UserConstructionScript`
  (locals (hemisphere :type "Float (double-precision)") (fanScaleZ :type "Float (double-precision)"))
  (bind _capsule (`self.Capsule`))
  (bind _capsule_2 (`self.Capsule`))
  (bind (_relativescale3d_x _relativescale3d_y _relativescale3d_z) (`KismetMathLibrary.BreakVector` (`SceneComponent.RelativeScale3D` (`self.Fan`))))
  (set `local.hemisphere` (- (`CapsuleComponent.GetUnscaledCapsuleHalfHeight` _capsule_2) (`CapsuleComponent.GetUnscaledCapsuleHalfHeight_WithoutHemisphere` _capsule_2)))
  (set `local.fanScaleZ` _relativescale3d_z)
  (`CapsuleComponent.SetCapsuleHalfHeight` _capsule (/ (* (+ (`self.Height`) (`local.hemisphere`)) 0.5) (`local.fanScaleZ`)) true)
  (`SceneComponent.K2_SetRelativeLocation` _capsule (`KismetMathLibrary.MakeVector` 0.0 0.0 (/ (* (- (`self.Height`) (`local.hemisphere`)) 0.5) (`local.fanScaleZ`))) false false))