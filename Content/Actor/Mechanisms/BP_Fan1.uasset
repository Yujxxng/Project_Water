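; BP_Fan1 is a fan mechanism that lifts the player character, triggered when it is in Vapor state inside the fan's capsule.
; The first Vapor tick after an overlap applies an upward impulse, then Tick adds vertical velocity with a cosine falloff up to Height, without rechecking the state.
; The construction script sizes and positions the capsule from Height.
; The arrow's Direction is stored but unused.
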(event `self.ReceiveBeginPlay`
  (bind _returnvalue (`GameplayStatics.GetPlayerCharacter` 0))
  (set `self.Direction` (`KismetMathLibrary.GetForwardVector` (`SceneComponent.K2_GetComponentRotation` (`self.Arrow`))))
  (set `self.PlayerMovement` (`Character.CharacterMovement` _returnvalue))
  (bind _asproject_water_character (cast `ProjectWaterCharacter` _returnvalue))
  (set `self.PlayerState` (`ProjectWaterCharacter.CharacterState` _asproject_water_character)))

(event `self.ReceiveActorBeginOverlap`
  (params (OtherActor :type "Actor Object Reference"))
  (set `self.bOverlapped` true)
  (set `self.bFirstVapor` true))

(event `self.ReceiveTick`
  (params (DeltaSeconds :type "Float (single-precision)"))
  (bind (_returnvalue_x _returnvalue_y _returnvalue_z) (`KismetMathLibrary.BreakVector` (`self.K2_GetActorLocation`)))
  (bind _playermovement (`self.PlayerMovement`))
  (bind (_returnvalue_x_2 _returnvalue_y_2 _returnvalue_z_2) (`KismetMathLibrary.BreakVector` (`self.K2_GetActorLocation` (`GameplayStatics.GetPlayerCharacter` 0))))
  (bind (_velocity_x _velocity_y _velocity_z) (`KismetMathLibrary.BreakVector` (`MovementComponent.Velocity` _playermovement)))
  (bind _returnvalue (- (- _returnvalue_z_2 91.0) (+ _returnvalue_z 120.0)))
  (if (`self.bOverlapped`)
    (if (`self.bFirstVapor`)
      (if (`|EnumEquality` (`CharacterState.State` (`self.PlayerState`)) "STATE_Vapor")
        (set `self.bFirstVapor` false)
        (`CharacterMovementComponent.AddImpulse` (`self.PlayerMovement`) (0.0 0.0 100.0) false)
        (if (< _returnvalue (`self.Height`)) :!label _label
          (set `MovementComponent.Velocity` (`KismetMathLibrary.MakeVector` _velocity_x _velocity_y (+ _velocity_z (* (`KismetMathLibrary.DegCos` (* (/ _returnvalue (`self.Height`)) 90.0)) 10.0))) _playermovement))
        (else
          (`KismetSystemLibrary.PrintString` "Hello")))
      (else
        (goto _label)))))

(event `self.ReceiveActorEndOverlap`
  (params (OtherActor :type "Actor Object Reference"))
  (set `self.bOverlapped` false))

(fn `UserConstructionScript`
  (bind _capsule (`self.Capsule`))
  (bind _height (`self.Height`))
  (`CapsuleComponent.SetCapsuleHalfHeight` _capsule (* (+ _height 80.0) 2.5) true)
  (`SceneComponent.K2_SetRelativeLocation` _capsule (`KismetMathLibrary.MakeVector` 0.0 0.0 (+ (* (- _height 80.0) 2.5) 120.0)) false false))