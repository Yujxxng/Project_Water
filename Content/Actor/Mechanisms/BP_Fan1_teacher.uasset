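; Fan mechanism actor that pushes the third-person player character along its Arrow direction and lets it float.
; Each tick a debug-drawn capsule trace runs from the Base up to MaxHeight, looking for pawns.
; Below half MaxHeight in world Z, the character receives a small impulse along the Arrow.
; At or above that height, a nearly stationary character gets near-zero gravity scale, which this graph never restores.
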(event `self.ReceiveTick`
  (params (DeltaSeconds :type "Float (single-precision)"))
  (bind _returnvalue (`SceneComponent.K2_GetComponentLocation` (`self.Base`)))
  (bind _returnvalue_2 (`KismetMathLibrary.GetForwardVector` (`SceneComponent.K2_GetComponentRotation` (`self.Arrow`))))
  (bind _outhit (`KismetSystemLibrary.CapsuleTraceSingleForObjects` :`Start` _returnvalue :`End` (+ _returnvalue (* _returnvalue_2 (`self.MaxHeight`))) :`ObjectTypes` (`|MakeArray` "ObjectTypeQuery3" :!type "EObjectTypeQuery Enum") :`DrawDebugType` "ForOneFrame"))
  (bind _asbp_third_person_character_yj (cast `/Game/ThirdPerson/Blueprints/BP_ThirdPersonCharacter_YJ` (`.HitActor` (`GameplayStatics.BreakHitResult` _outhit))))
  (bind (_returnvalue_x _returnvalue_y _returnvalue_z) (`KismetMathLibrary.BreakVector` (`self.K2_GetActorLocation` _asbp_third_person_character_yj)))
  (if (>= _returnvalue_z (* (`self.MaxHeight`) 0.5))
    (bind _charactermovement (`Character.CharacterMovement` _asbp_third_person_character_yj))
    (if (<= (`KismetMathLibrary.VSize` (`self.GetVelocity` (`PawnMovementComponent.GetPawnOwner` _charactermovement))) 3.0)
      (set `CharacterMovementComponent.GravityScale` 0.01 _charactermovement))
    (else
      (`CharacterMovementComponent.AddImpulse` _charactermovement (* _returnvalue_2 (`KismetMathLibrary.RandomFloatInRange` 6.0 6.0)) false))))

(fn `UserConstructionScript`)