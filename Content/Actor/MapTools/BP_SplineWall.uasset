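; BP_SplineWall is a map tool actor that builds a wall of repeated meshes along a spline.
; Its construction script assigns WallMesh to an instanced static mesh and spaces instances by the mesh's X bounding length along the spline.
; Each unscaled instance points its X axis at the next sample point.
; Spline height is ignored: every local-space instance takes its Z from the actor's world Z, keeping the wall level.
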(fn `GetIndexLocation`
  (params (idx :type Integer))
  (returns (Location :type "Vector Structure"))
  (bind (_returnvalue_x _returnvalue_y) (`KismetMathLibrary.BreakVector` (`SplineComponent.GetLocationAtDistanceAlongSpline` (`self.Spline`) (* idx (`self.MeshLength`)) "Local")))
  (return (`KismetMathLibrary.MakeVector` _returnvalue_x _returnvalue_y (`self.BottomZ`))))

(fn `UserConstructionScript`
  (bind (_returnvalue_x _returnvalue_y _returnvalue_z) (`KismetMathLibrary.BreakVector` (`self.K2_GetActorLocation`)))
  (bind _wallmesh (`self.WallMesh`))
  (bind (_min _max) (break `Box` (`StaticMesh.GetBoundingBox` _wallmesh)))
  (bind _returnvalue_x_2 (`KismetMathLibrary.BreakVector` (- _max _min)))
  (set `self.BottomZ` _returnvalue_z)
  (`StaticMeshComponent.SetStaticMesh` (`self.InstancedStaticMesh`) _wallmesh)
  (bind _output_get (set `self.MeshLength` _returnvalue_x_2))
  (for _index (range (+ (`KismetMathLibrary.FFloor` (/ (`SplineComponent.GetSplineLength` (`self.Spline`)) _output_get)) 1))
    (bind _location (`self.GetIndexLocation` _index))
    (bind _location_2 (`self.GetIndexLocation` (+ _index 1)))
    (`InstancedStaticMeshComponent.AddInstance` (`self.InstancedStaticMesh`) (`KismetMathLibrary.MakeTransform` _location (`KismetMathLibrary.MakeRotFromX` (- _location_2 _location))) false)))