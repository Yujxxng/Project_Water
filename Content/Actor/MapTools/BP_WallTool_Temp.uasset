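; BP_WallTool_Temp is a map-building tool actor that fills a wall area with copies of a chosen static mesh.
; The construction script divides the Corner vector's X and Z by the mesh's bounding-box size to get column and row counts.
; Nested loops then add local-space HierarchicalInstancedStaticMesh instances on that X-Z grid, spaced edge to edge by mesh size.
; BeginPlay only prints the two computed counts.
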(event `self.ReceiveBeginPlay`
  (bind (_corner_x _corner_y _corner_z) (`KismetMathLibrary.BreakVector` (`self.Corner`)))
  (bind (_min _max) (break `Box` (`StaticMesh.GetBoundingBox` (`self.StaticMesh`))))
  (bind (_returnvalue_x _returnvalue_y _returnvalue_z) (`KismetMathLibrary.BreakVector` (- _max _min)))
  (`KismetSystemLibrary.PrintString` (`KismetStringLibrary.Conv_IntToString` (`KismetMathLibrary.FFloor` (/ _corner_x _returnvalue_x))))
  (`KismetSystemLibrary.PrintString` (`KismetStringLibrary.Conv_IntToString` (`KismetMathLibrary.FFloor` (/ _corner_z _returnvalue_z)))))

(fn `UserConstructionScript`
  (bind _staticmesh (`self.StaticMesh`))
  (bind (_corner_x _corner_y _corner_z) (`KismetMathLibrary.BreakVector` (`self.Corner`)))
  (bind (_min _max) (break `Box` (`StaticMesh.GetBoundingBox` _staticmesh)))
  (bind (_returnvalue_x _returnvalue_y _returnvalue_z) (`KismetMathLibrary.BreakVector` (- _max _min)))
  (`StaticMeshComponent.SetStaticMesh` (`self.HierarchicalInstancedStaticMesh`) _staticmesh)
  (for _index (range (+ (`KismetMathLibrary.FFloor` (/ _corner_x _returnvalue_x)) 1))
    (for _index_2 (range (+ (`KismetMathLibrary.FFloor` (/ _corner_z _returnvalue_z)) 1))
      (`InstancedStaticMeshComponent.AddInstance` (`self.HierarchicalInstancedStaticMesh`) (`KismetMathLibrary.MakeTransform` (`KismetMathLibrary.MakeVector` (* _returnvalue_x _index) 0.0 (* _index_2 _returnvalue_z))) false))))