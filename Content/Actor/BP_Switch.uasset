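; BP_Switch is an interactable switch that starts and stops a referenced moving platform.
; Each Interact event flips the IsPlatformMove flag, enables or disables tick on the platform's InterpToMovement component to match, and prints on or off.
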(event `/Game/Actor/BPI_Interact.Interact`
  (if (not (`self.is Platform move?`))
    (set `self.is Platform move?` true)
    (`KismetSystemLibrary.PrintString` "on")
    (`ActorComponent.SetComponentTickEnabled` (`/Game/Actor/BP_MovingPlatform.InterpToMovement` (`self.Platform`)) true)
    (else
      (set `self.is Platform move?` false)
      (`KismetSystemLibrary.PrintString` "off")
      (`ActorComponent.SetComponentTickEnabled` (`/Game/Actor/BP_MovingPlatform.InterpToMovement` (`self.Platform`)) false))))

(fn `UserConstructionScript`)