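; BP_Orb is an interactable pickup that unlocks a character state for the player.
; A widget, hidden at BeginPlay, shows while anything overlaps the Box, with no filtering by actor, and hides when an overlap ends.
; Interact plays a 2D orb sound, casts the player to BP_ThirdPersonCharacter_YJ, passes the orb's State to CharacterState.UnlockState, then destroys the orb.
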(event `self.ReceiveBeginPlay`
  (`SceneComponent.SetVisibility` (`self.Widget`) false false))

(event `/Game/Actor/InteractActors/BPI_Interact.Interact`
  (`GameplayStatics.PlaySound2D` "/Game/Sound/SFX/sfx_orb.sfx_orb" 1.0 1.0 0.0 null null)
  (bind _asbp_third_person_character_yj (cast `/Game/ThirdPerson/Blueprints/BP_ThirdPersonCharacter_YJ` (`GameplayStatics.GetPlayerCharacter` 0)))
  (`CharacterState.UnlockState` (`ProjectWaterCharacter.CharacterState` _asbp_third_person_character_yj) (`self.State`))
  (`self.K2_DestroyActor`))

(event `self.Box.OnComponentBeginOverlap`
  (params (OverlappedComponent :type "PrimitiveComponent Object Reference") (OtherActor :type "Actor Object Reference") (OtherComp :type "PrimitiveComponent Object Reference") (OtherBodyIndex :type Integer) (bFromSweep :type Boolean) (SweepResult :type "HitResult Structure (by ref)"))
  (`SceneComponent.SetVisibility` (`self.Widget`) true false))

(event `self.Box.OnComponentEndOverlap`
  (params (OverlappedComponent :type "PrimitiveComponent Object Reference") (OtherActor :type "Actor Object Reference") (OtherComp :type "PrimitiveComponent Object Reference") (OtherBodyIndex :type Integer))
  (`SceneComponent.SetVisibility` (`self.Widget`) false false))

(fn `UserConstructionScript`)