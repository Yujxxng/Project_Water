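; Pushable block that the player shoves in fixed grid steps by walking squarely into it.
; CanPush uses line and box traces to require the player facing it, a clear path, floor ahead, nothing on top, and no falling.
; On hit, it locks movement, widens the capsule, attaches the player and plays a montage whose notify starts a timeline-driven move.
; Steps repeat while W is held; StopPushing then restores the player.
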(event `self.ReceiveTick`
  (params (DeltaSeconds :type "Float (single-precision)")))

(event `self.ReceiveHit`
  (params (MyComp :type "PrimitiveComponent Object Reference") (Other :type "Actor Object Reference") (OtherComp :type "PrimitiveComponent Object Reference") (bSelfMoved :type Boolean) (HitLocation :type "Vector Structure") (HitNormal :type "Vector Structure") (NormalImpulse :type "Vector Structure") (Hit :type "HitResult Structure (by ref)"))
  (bind _returnvalue (`self.GetActorForwardVector` Other))
  (bind _returnvalue_2 (`GameplayStatics.GetPlayerCharacter` 0))
  (bind _capsulecomponent (`Character.CapsuleComponent` _returnvalue_2))
  (bind _mesh (`Character.Mesh` (`GameplayStatics.GetPlayerCharacter` 0)))
  (if (== (`GameplayStatics.GetPlayerCharacter` 0) Other)
    (if (> (`KismetMathLibrary.Dot_VectorVector` HitNormal _returnvalue) 0.93)
      (set `self.Pushable Direction` (`KismetMathLibrary.MakeVector` (`KismetMathLibrary.Conv_IntToDouble` (`KismetMathLibrary.Round` (.x _returnvalue))) (`KismetMathLibrary.Conv_IntToDouble` (`KismetMathLibrary.Round` (.y _returnvalue))) (`KismetMathLibrary.Conv_IntToDouble` (`KismetMathLibrary.Round` (.z _returnvalue)))))
      (bind _canpush (`self.Can Push`))
      (if _canpush
        (`CharacterMovementComponent.DisableMovement` (`Character.CharacterMovement` _returnvalue_2))
        (`CapsuleComponent.SetCapsuleRadius` _capsulecomponent 65.0 true)
        (`KismetSystemLibrary.MoveComponentTo` _capsulecomponent (+ (`SceneComponent.K2_GetComponentLocation` _capsulecomponent) (* (`self.GetActorForwardVector` _returnvalue_2) -45.0)) (`SceneComponent.K2_GetComponentRotation` _capsulecomponent))
        (`self.K2_AttachToActor` (`GameplayStatics.GetPlayerCharacter` 0) self "None" "KeepWorld" "KeepWorld" "KeepWorld" true)
        (if (`AnimInstance.IsAnyMontagePlaying` (`SkeletalMeshComponent.GetAnimInstance` _mesh))
          (`/Engine/EditorBlueprintResources/StandardMacros.Gate` true :!label _label
            (:`Exit`
              (`self.Push`)))
          (else
            (`|PlayMontage` _mesh "/Game/Characters/Push/AM_PushMongtage.AM_PushMongtage" 2.0
              (:`OnNotifyBegin`
                (`self.Push`)
                (goto _label :!via `Open`)))))))))

(event `Push`
  (bind _canpush (`self.Can Push`))
  (if _canpush
    (set `self.Current Location` (`self.K2_GetActorLocation`))
    (bind (_direction _position) (`Timeline|MoveBlock` :!via `PlayFromStart`)
      (:`Update`
        (`self.K2_SetActorRelativeLocation` (+ (`self.Current Location`) (* _position (`self.Pushable Direction`) (`self.Travel Distance`)))))
      (:`Finished`
        (if (`PlayerController.IsInputKeyDown` (`GameplayStatics.GetPlayerController` 0) "W")
          (bind _canpush_2 (`self.Can Push`))
          (if _canpush_2
            (`self.Push`)
            (else
              (`self.StopPushing`)))
          (else
            (`self.StopPushing`)))))
    (else
      (`self.StopPushing`))))

(event `StopPushing`
  (bind _returnvalue (`GameplayStatics.GetPlayerCharacter` 0))
  (`|PlayMontage` (`Character.Mesh` (`GameplayStatics.GetPlayerCharacter` 0)) "/Game/Characters/Push/AM_PushMongtage.AM_PushMongtage" 2.0 0.0 "End"
    (:`OnCompleted`
      (`CharacterMovementComponent.SetMovementMode` (`Character.CharacterMovement` _returnvalue) "MOVE_Walking" 0)
      (`self.K2_DetachFromActor` _returnvalue "KeepWorld" "KeepWorld" "KeepWorld")
      (`CapsuleComponent.SetCapsuleRadius` (`Character.CapsuleComponent` _returnvalue) 35.0 true))))

(fn `Can Push`
  (returns (CanPush :type Boolean))
  (bind _returnvalue (`self.K2_GetActorLocation`))
  (bind _returnvalue_2 (`GameplayStatics.GetPlayerCharacter` 0))
  (bind _sphere (`self.Sphere`))
  (bind _returnvalue_3 (`self.K2_GetActorLocation` _returnvalue_2))
  (bind _returnvalue_4 (+ (`self.K2_GetActorLocation`) (0.0 0.0 200.0)))
  (bind (_returnvalue_origin _returnvalue_boxextent) (`KismetMathLibrary.BreakBoxSphereBounds` (`StaticMesh.GetBounds` (`StaticMeshComponent.StaticMesh` _sphere))))
  (bind _returnvalue_5 (+ (`self.K2_GetActorLocation`) (* (`self.Pushable Direction`) (`self.Travel Distance`) 1.5) (0.0 0.0 100.0)))
  (bind (_outhit _returnvalue_6) (`KismetSystemLibrary.LineTraceSingle` _returnvalue_3 (+ _returnvalue_3 (* (`self.GetActorForwardVector` _returnvalue_2) 100.0)) "TraceTypeQuery1" false (`|MakeArray` _returnvalue_2 :!type "Actor Object Reference") "ForDuration" false))
  (if _returnvalue_6
    (if (== (`.HitActor` (`GameplayStatics.BreakHitResult` _outhit)) self)
      (bind (_outhit_2 _returnvalue_7) (`KismetSystemLibrary.BoxTraceSingle` :`Start` (+ _returnvalue (0.0 0.0 100.0)) :`End` (+ _returnvalue (* (`self.Pushable Direction`) (`self.Travel Distance`)) (0.0 0.0 100.0)) :`HalfSize` (* _returnvalue_boxextent (`SceneComponent.RelativeScale3D` _sphere) (0.8 0.8 0.8)) :`TraceChannel` "TraceTypeQuery2" :`DrawDebugType` "Persistent" :`TraceHitColor` (struct :`G` 1.0 :`B` 0.940764 :`A` 1.0)))
      (`KismetSystemLibrary.PrintString` (`KismetSystemLibrary.GetDisplayName` (`.HitActor` (`GameplayStatics.BreakHitResult` _outhit_2))))
      (if (not _returnvalue_7)
        (bind (_outhit_3 _returnvalue_8) (`KismetSystemLibrary.LineTraceSingle` :`Start` _returnvalue_5 :`End` (+ _returnvalue_5 (0.0 0.0 -200.0)) :`TraceChannel` "TraceTypeQuery1" :`DrawDebugType` "ForDuration" :`TraceColor` (struct :`R` 0.076735 :`B` 1.0 :`A` 1.0) :`TraceHitColor` (struct :`R` 0.995748 :`G` 1.0 :`A` 1.0)))
        (if _returnvalue_8
          (bind (_outhit_4 _returnvalue_9) (`KismetSystemLibrary.LineTraceSingle` :`Start` _returnvalue_4 :`End` (+ _returnvalue_4 (0.0 0.0 200.0)) :`TraceChannel` "TraceTypeQuery1" :`TraceHitColor` (struct :`R` 0.9878 :`B` 1.0 :`A` 1.0)))
          (if _returnvalue_9
            (return false)
            (elif (`NavMovementComponent.IsFalling` (`Character.CharacterMovement` (`GameplayStatics.GetPlayerCharacter` 0)))
              (return false)
              (else
                (return true))))
          (else
            (return false)))
        (else
          (return false)))
      (else
        (return false)))
    (else
      (return false))))

(fn `UserConstructionScript`)