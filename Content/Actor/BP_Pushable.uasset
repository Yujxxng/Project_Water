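; Pushable actor that the player shoves in fixed-distance steps by walking squarely into it.
; On hit, the rounded player forward sets the direction, and line and box traces validate the push, exempting an obstacle named "Cube" as a ramp.
; The player's movement is disabled, capsule widened and character attached while a montage notify starts the MoveBlock timeline.
; Steps repeat while W is held, then the montage's End section restores the player.
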(event `self.ReceiveHit`
  (params (MyComp :type "PrimitiveComponent Object Reference") (Other :type "Actor Object Reference") (OtherComp :type "PrimitiveComponent Object Reference") (bSelfMoved :type Boolean) (HitLocation :type "Vector Structure") (HitNormal :type "Vector Structure") (NormalImpulse :type "Vector Structure") (Hit :type "HitResult Structure (by ref)"))
  (bind _returnvalue (`self.GetActorForwardVector` Other))
  (bind _returnvalue_2 (`GameplayStatics.GetPlayerCharacter` 0))
  (bind _capsulecomponent (`Character.CapsuleComponent` _returnvalue_2))
  (bind _mesh (`Character.Mesh` (`GameplayStatics.GetPlayerCharacter` 0)))
  (if (== (`GameplayStatics.GetPlayerCharacter` 0) Other)
    (if (> (`KismetMathLibrary.Dot_VectorVector` HitNormal _returnvalue) 0.93)
      (set `self.Pushable Direction` (`KismetMathLibrary.MakeVector` (`KismetMathLibrary.Conv_IntToDouble` (`KismetMathLibrary.Round` (.x _returnvalue))) (`KismetMathLibrary.Conv_IntToDouble` (`KismetMathLibrary.Round` (.y _returnvalue))) (`KismetMathLibrary.Conv_IntToDouble` (`KismetMathLibrary.Round` (.z _returnvalue)))))
      (bind _canpush (`self.Can Push`))
      (if _canpush
        (`CharacterMovementComponent.DisableMovement` (`Character.CharacterMovement` _returnvalue_2))
        (`CapsuleComponent.SetCapsuleRadius` _capsulecomponent 65.0 true)
        (`KismetSystemLibrary.MoveComponentTo` _capsulecomponent (+ (`SceneComponent.K2_GetComponentLocation` _capsulecomponent) (* (`self.GetActorForwardVector` _returnvalue_2) -45.0)) (`SceneComponent.K2_GetComponentRotation` _capsulecomponent))
        (`self.K2_AttachToActor` (`GameplayStatics.GetPlayerCharacter` 0) self "None" "KeepWorld" "KeepWorld" "KeepWorld" true)
        (if (`AnimInstance.IsAnyMontagePlaying` (`SkeletalMeshComponent.GetAnimInstance` _mesh))
          (`/Engine/EditorBlueprintResources/StandardMacros.Gate` true :!label _label
            (:`Exit`
              (`self.Push`)))
          (else
            (`|PlayMontage` _mesh "/Game/Characters/Push/AM_PushMongtage.AM_PushMongtage"
              (:`OnNotifyBegin`
                (`self.Push`)
                (goto _label :!via `Open`)))))))))

(event `Push`
  (set `self.Current Location` (`self.K2_GetActorLocation`))
  (bind (_direction _position) (`Timeline|MoveBlock` :!via `PlayFromStart`)
    (:`Update`
      (`self.K2_SetActorRelativeLocation` (+ (`self.Current Location`) (* _position (`self.Pushable Direction`) (`self.Travel Distance`)))))
    (:`Finished`
      (if (`PlayerController.IsInputKeyDown` (`GameplayStatics.GetPlayerController` 0) "W")
        (`self.Push`)
        (else
          (`self.StopPushing`))))))

(event `StopPushing`
  (bind _returnvalue (`GameplayStatics.GetPlayerCharacter` 0))
  (`|PlayMontage` (`Character.Mesh` (`GameplayStatics.GetPlayerCharacter` 0)) "/Game/Characters/Push/AM_PushMongtage.AM_PushMongtage" 1.0 0.0 "End"
    (:`OnCompleted`
      (`CharacterMovementComponent.SetMovementMode` (`Character.CharacterMovement` _returnvalue) "MOVE_Walking" 0)
      (`self.K2_DetachFromActor` _returnvalue "KeepWorld" "KeepWorld" "KeepWorld")
      (`CapsuleComponent.SetCapsuleRadius` (`Character.CapsuleComponent` _returnvalue) 35.0 true))))

(fn `Can Push`
  (returns (CanPush :type Boolean))
  (bind _returnvalue (`GameplayStatics.GetPlayerCharacter` 0))
  (bind _returnvalue_2 (`self.K2_GetActorLocation`))
  (bind _sphere (`self.Sphere`))
  (bind _returnvalue_3 (`self.K2_GetActorLocation` _returnvalue))
  (bind (_returnvalue_origin _returnvalue_boxextent) (`KismetMathLibrary.BreakBoxSphereBounds` (`StaticMesh.GetBounds` (`StaticMeshComponent.StaticMesh` _sphere))))
  (bind (_outhit _returnvalue_4) (`KismetSystemLibrary.LineTraceSingle` _returnvalue_3 (+ _returnvalue_3 (* (`self.GetActorForwardVector` _returnvalue) 100.0)) "TraceTypeQuery1" false (`|MakeArray` _returnvalue :!type "Actor Object Reference") "ForOneFrame" false))
  (if _returnvalue_4
    (if (== (`.HitActor` (`GameplayStatics.BreakHitResult` _outhit)) self)
      (bind (_outhit_2 _returnvalue_5) (`KismetSystemLibrary.BoxTraceSingle` :`Start` (+ _returnvalue_2 (0.0 0.0 0.0)) :`End` (+ _returnvalue_2 (* (`self.Pushable Direction`) (`self.Travel Distance`)) (0.0 0.0 0.0)) :`HalfSize` (* _returnvalue_boxextent (`SceneComponent.RelativeScale3D` _sphere) (0.8 0.8 0.8)) :`TraceChannel` "TraceTypeQuery1" :`DrawDebugType` "ForDuration"))
      ;[1 1 1] If ramp, can push
      (if (`KismetStringLibrary.EqualEqual_StrStr` (`KismetSystemLibrary.GetDisplayName` (`.HitActor` (`GameplayStatics.BreakHitResult` _outhit_2))) "Cube")
        (return true)
        (else
          (return (not _returnvalue_5))))
      (else
        (return false)))
    (else
      (return false))))

(fn `UserConstructionScript`)