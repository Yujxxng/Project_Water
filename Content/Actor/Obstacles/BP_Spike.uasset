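; BP_Spike is a spike obstacle that damages the ProjectWaterCharacter on entering its box and knocks the player back.
; Any overlap sets a flag, cleared on end overlap, that makes Tick repeatedly push player 0 away from an offset actor origin.
; The construction script applies spike mesh and scale and loops over a grid sized from the plane and mesh bounds, but its AddInstance step is disconnected.
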(event `self.Box.OnComponentBeginOverlap`
  (params (OverlappedComponent :type "PrimitiveComponent Object Reference") (OtherActor :type "Actor Object Reference") (OtherComp :type "PrimitiveComponent Object Reference") (OtherBodyIndex :type Integer) (bFromSweep :type Boolean) (SweepResult :type "HitResult Structure (by ref)"))
  (set `self.NewVar` true)
  (bind _asproject_water_character (cast `ProjectWaterCharacter` OtherActor))
  (`GameplayStatics.ApplyDamage` _asproject_water_character 1.0 null null "/Script/Engine.DamageType"))

(event `self.ReceiveTick`
  (params (DeltaSeconds :type "Float (single-precision)"))
  (bind _returnvalue (`GameplayStatics.GetPlayerCharacter` 0))
  (if (`self.NewVar`)
    (`CharacterMovementComponent.AddImpulse` (`Character.CharacterMovement` _returnvalue) (* (- (`self.K2_GetActorLocation` _returnvalue) (+ (`self.K2_GetActorLocation`) (100.0 100.0 0.0))) 20.0) false)))

(event `self.Box.OnComponentEndOverlap`
  (params (OverlappedComponent :type "PrimitiveComponent Object Reference") (OtherActor :type "Actor Object Reference") (OtherComp :type "PrimitiveComponent Object Reference") (OtherBodyIndex :type Integer))
  (set `self.NewVar` false))

(fn `UserConstructionScript`
  (locals (Spacing :type "Float (double-precision)"))
  (bind _spike (`self.Spike`))
  (bind _returnvalue_x (`KismetMathLibrary.BreakVector` (`SceneComponent.K2_GetComponentScale` (`self.Plane`))))
  (bind (_min _max) (break `Box` (`StaticMesh.GetBoundingBox` (`self.SpikeSM`))))
  (bind _returnvalue_x_2 (`KismetMathLibrary.BreakVector` (* (- _max _min) 0.24)))
  (`SceneComponent.SetWorldScale3D` _spike (`KismetMathLibrary.Conv_DoubleToVector` (`self.SpikeScale`)))
  (`StaticMeshComponent.SetStaticMesh` _spike (`self.SpikeSM`))
  (bind _output_get (set `local.Spacing` (+ (`self.Offset`) _returnvalue_x_2)))
  (bind _returnvalue (`KismetMathLibrary.FTrunc` (/ (* _returnvalue_x 100.0) _output_get)))
  (for _index (range 1 (+ _returnvalue 1))
    (for _index_2 (range 1 (+ _returnvalue 1))
      _)))