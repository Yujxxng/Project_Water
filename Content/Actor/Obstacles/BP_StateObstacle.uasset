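; BP_StateObstacle is an obstacle that damages ProjectWaterCharacter actors unless their character state is on its ignore list.
; Each Tick it checks the characters overlapping its Box against IgnoredStates, which SetIgnoredStates appends to.
; A one-second Delay inside the loop precedes DamageHearts and a debug print of hearts, so calls during a pending delay are dropped.
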(event `self.ReceiveTick`
  (params (DeltaSeconds :type "Float (single-precision)"))
  (for _array_element (`PrimitiveComponent.GetOverlappingActors` (`self.Box`) "/Script/ProjectWater.ProjectWaterCharacter")
    (bind _asproject_water_character (cast `ProjectWaterCharacter` _array_element))
    (if (not (`BlueprintSetLibrary.Set_Contains` (`self.IgnoredStates`) (`CharacterState.State` (`ProjectWaterCharacter.CharacterState` _asproject_water_character))))
      (`KismetSystemLibrary.Delay` 1.0)
      (`ProjectWaterCharacter.DamageHearts` _asproject_water_character (`self.Damage`))
      (bind _returnvalue (`ProjectWaterCharacter.GetHearts` _asproject_water_character))
      (`KismetSystemLibrary.PrintString` (`KismetStringLibrary.Conv_IntToString` _returnvalue)))))

(fn `SetIgnoredStates`
  (params (State :type "EState Enum" :default "STATE_None"))
  (`BlueprintSetLibrary.Set_Add` (`self.IgnoredStates`) State))

(fn `UserConstructionScript`)