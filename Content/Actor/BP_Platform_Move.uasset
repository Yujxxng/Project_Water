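; BP_Platform_Move is a platform actor that moves along the forward direction of its Arrow component.
; On BeginPlay it records its start location, applies MoveSpeed as the MovementGraph timeline play rate, and plays the timeline after DelayTime.
; Each timeline update offsets the start location by the Arrow's forward vector scaled by MovementValue and Distance, setting the location without sweep.
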(event `self.ReceiveBeginPlay`
  (set `self.initialLocation` (`self.K2_GetActorLocation`))
  (`TimelineComponent.SetPlayRate` (`self.MovementGraph`) (`self.moveSpeed`))
  (`KismetSystemLibrary.Delay` (`self.delayTime`))
  (bind (_direction _movementvalue) (`Timeline|MovementGraph`)
    (:`Update`
      (`self.K2_SetActorLocation` (+ (`self.initialLocation`) (* (`SceneComponent.GetForwardVector` (`self.Arrow`)) (* _movementvalue (`self.distance`))))))))

(fn `UserConstructionScript`)