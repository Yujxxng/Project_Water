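; BP_WorldRoad1 is a world actor that lays a road by repeating RoadMesh along a spline.
; The construction script derives spacing from the mesh's bounding-box X size plus Offset, then fits the instance count to the spline length.
; Each instanced static mesh sits at its local-space spline distance, rotated toward the next point at unit scale, without bending.
; The event graph has no active logic.
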(fn `GetLocation`
  (params (A :type "Float (double-precision)"))
  (returns (ReturnValue :type "Vector Structure"))
  (return (`SplineComponent.GetLocationAtDistanceAlongSpline` (`self.Spline`) (* A (`self.Spacing`)) "Local")))

(fn `UserConstructionScript`
  (locals (NumMesh :type Integer :default 0))
  (bind (_min _max) (break `Box` (`StaticMesh.GetBoundingBox` (`self.RoadMesh`))))
  (bind _returnvalue_x (`KismetMathLibrary.BreakVector` (- _max _min)))
  (`StaticMeshComponent.SetStaticMesh` (`self.InstancedStaticMesh`) (`self.RoadMesh`))
  (bind _output_get (set `self.Spacing` (+ (`self.Offset`) _returnvalue_x)))
  (bind _output_get_2 (set `local.NumMesh` (`KismetMathLibrary.FFloor` (/ (`SplineComponent.GetSplineLength` (`self.Spline`)) _output_get))))
  (for _index (range (+ _output_get_2 1))
    (bind _returnvalue (`self.GetLocation` (`KismetMathLibrary.Conv_IntToDouble` _index)))
    (bind _returnvalue_2 (`self.GetLocation` (`KismetMathLibrary.Conv_IntToDouble` (+ _index 1))))
    (`InstancedStaticMeshComponent.AddInstance` (`self.InstancedStaticMesh`) (`KismetMathLibrary.MakeTransform` _returnvalue (`KismetMathLibrary.MakeRotFromX` (- _returnvalue_2 _returnvalue))) false)))