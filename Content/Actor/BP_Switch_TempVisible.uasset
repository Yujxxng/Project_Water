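; Switch actor that temporarily makes every BP_Platform_Basic actor in the level visible and solid when interacted with.
; Interact is ignored while IsPlatformVisible is set; otherwise it sets the flag, enables collision and unhides each platform.
; A three-second Delay, triggered from inside the loop, then clears the flag, disables collision and hides all platforms again, with debug prints for on and off.
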(event `self.Interact`
  (if (not (`self.isPlatformVisible`))
    (set `self.isPlatformVisible` true)
    (`KismetSystemLibrary.PrintString` "on")
    (bind _outactors (`GameplayStatics.GetAllActorsOfClass` "/Game/Actor/BP_Platform_Basic.BP_Platform_Basic_C"))
    (for _array_element _outactors
      (`|ExecutionSequence`
        (:`then_0`
          (`self.SetActorEnableCollision` _array_element true))
        (:`then_1`
          (`self.SetActorHiddenInGame` _array_element false)))
      (`KismetSystemLibrary.Delay` 3.0)
      (set `self.isPlatformVisible` false)
      (`KismetSystemLibrary.PrintString` "off")
      (bind _outactors_2 (`GameplayStatics.GetAllActorsOfClass` "/Game/Actor/BP_Platform_Basic.BP_Platform_Basic_C"))
      (for _array_element_2 _outactors_2
        (`|ExecutionSequence`
          (:`then_0`
            (`self.SetActorEnableCollision` _array_element_2 false))
          (:`then_1`
            (`self.SetActorHiddenInGame` _array_element_2 true)))))))

(fn `UserConstructionScript`)