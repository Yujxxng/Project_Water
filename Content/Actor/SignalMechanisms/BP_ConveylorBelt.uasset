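; Conveyor belt signal mechanism actor that pushes whatever sits on it along a fixed direction.
; BeginPlay caches the Arrow's forward vector, and Tick offsets every actor overlapping the Box along it by Speed, scaled by delta time, without sweeping.
; Activate and Inactivate flip the Sign to reverse the travel direction and roll or yaw the static mesh half a turn to match, so the belt never stops.
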(event `self.ReceiveBeginPlay`
  (set `self.InitialArrow` (`KismetMathLibrary.GetForwardVector` (`SceneComponent.K2_GetComponentRotation` (`self.Arrow`)))))

(event `self.ReceiveTick`
  (params (DeltaSeconds :type "Float (single-precision)"))
  (for _array_element (`PrimitiveComponent.GetOverlappingActors` (`self.Box`) null)
    (`self.K2_AddActorWorldOffset` _array_element (* (* DeltaSeconds (`self.Speed`)) (* (`self.InitialArrow`) (`self.Sign`))) false false)))

(fn `Activate`
  (set `self.Sign` -1)
  (`SceneComponent.K2_SetRelativeRotation` (`self.StaticMesh`) (struct :`Yaw` 180.0) false false))

(fn `Inactivate`
  (set `self.Sign` 1)
  (`SceneComponent.K2_SetRelativeRotation` (`self.StaticMesh`) (struct) false false))

(fn `UserConstructionScript`
  (`parent.UserConstructionScript`))