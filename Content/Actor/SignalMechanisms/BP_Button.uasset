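; BP_Button is a one-shot pressure plate that emits a signal when pressed.
; When an actor tagged Pressable overlaps its Trigger, it latches an Activated flag, calls EmitOnSignal and plays the PlatePressure timeline, which lerps the Plate's relative Z downward.
; Nothing in the graph resets the flag or raises the plate, so later overlaps are ignored.
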(event `self.Trigger.OnComponentBeginOverlap`
  (params (OverlappedComponent :type "PrimitiveComponent Object Reference") (OtherActor :type "Actor Object Reference") (OtherComp :type "PrimitiveComponent Object Reference") (OtherBodyIndex :type Integer) (bFromSweep :type Boolean) (SweepResult :type "HitResult Structure (by ref)"))
  (if (and (`self.ActorHasTag` OtherActor "Pressable") (not (`self.bActivated`)))
    (set `self.bActivated` true)
    (`self.EmitOnSignal`)
    (bind (_direction _height) (`Timeline|Plate Pressure`)
      (:`Update`
        (`SceneComponent.K2_SetRelativeLocation` (`self.Plate`) (`KismetMathLibrary.MakeVector` 0.0 0.0 (`KismetMathLibrary.Lerp` 5.0 -5.0 _height)) false false)))))

(fn `UserConstructionScript`)