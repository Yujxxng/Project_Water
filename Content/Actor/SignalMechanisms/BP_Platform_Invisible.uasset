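; Signal-mechanism platform that appears and becomes solid when activated, and turns invisible and non-colliding when inactivated.
; Activate and Inactivate only set the Visible flag and print an on/off debug string.
; Tick applies that flag every frame to the static mesh's visibility and the actor's collision, rather than updating them when the state changes.
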(event `self.ReceiveTick`
  (params (DeltaSeconds :type "Float (single-precision)"))
  (bind _visible (`self.Visible`))
  (`SceneComponent.SetVisibility` (`self.StaticMesh`) _visible false)
  (`self.SetActorEnableCollision` _visible))

(fn `Activate`
  (set `self.Visible` true)
  (`KismetSystemLibrary.PrintString` "on"))

(fn `Inactivate`
  (set `self.Visible` false)
  (`KismetSystemLibrary.PrintString` "off"))

(fn `UserConstructionScript`
  (`parent.UserConstructionScript`))