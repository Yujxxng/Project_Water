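; Timed platform in the signal mechanisms set that appears with collision for a set Duration when activated, then disappears.
; Activate only sets the Visible flag, which Tick polls to show the actor and start a Delay.
; When the Delay ends, the flag clears and the actor is hidden without collision, which is also its state whenever Visible is false.
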(event `self.ReceiveBeginPlay`)

(event `self.ReceiveTick`
  (params (DeltaSeconds :type "Float (single-precision)"))
  (if (`self.bVisible`)
    (`self.SetActorHiddenInGame` false)
    (`self.SetActorEnableCollision` true)
    (`KismetSystemLibrary.Delay` (`self.Duration`))
    (set `self.bVisible` false))
  (`self.SetActorHiddenInGame` true)
  (`self.SetActorEnableCollision` false))

(fn `Activate`
  (set `self.bVisible` true))

(fn `UserConstructionScript`
  (`parent.UserConstructionScript`))