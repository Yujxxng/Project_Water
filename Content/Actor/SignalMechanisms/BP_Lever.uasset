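; BP_Lever is a toggle lever in the signal mechanism system that emits on and off signals when interacted with.
; Each interaction flips the Activated state, emits the matching signal, and plays or reverses the RotateJoint timeline.
; The timeline scales Angle to swing the Joint's pitch, and BeginPlay starts the Joint pitched to negative Angle.
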(event `self.ReceiveBeginPlay`
  (`SceneComponent.K2_SetRelativeRotation` (`self.Joint`) (`KismetMathLibrary.MakeRotator` 0.0 (* (`self.Angle`) -1.0)) false false))

(event `/Game/Actor/BPI_Interact.Interact`
  (if (not (`self.bActivated`))
    (set `self.bActivated` true)
    (`self.EmitOnSignal`)
    (bind (_direction _rotationvalue) (`Timeline|RotateJoint` :!label _label)
      (:`Update`
        (`SceneComponent.K2_SetRelativeRotation` (`self.Joint`) (`KismetMathLibrary.MakeRotator` 0.0 (* _rotationvalue (`self.Angle`))) false false)))
    (else
      (set `self.bActivated` false)
      (`self.EmitOffSignal`)
      (goto _label :!via `Reverse`))))

(fn `UserConstructionScript`
  (`parent.UserConstructionScript`))