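; Pushable cube that the player shoves in TravelDistance steps by walking squarely into a face near its center.
; On hit it locks and attaches the player, then a timeline slides it, repeating while W is held.
; CanPush box-traces for obstacles and ground; a ledge releases the player and enables physics, with Tick clearing Falling once ground is found.
; Box overlap disables physics while the player is near, unless falling.
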(event `self.ReceiveHit`
  (params (MyComp :type "PrimitiveComponent Object Reference") (Other :type "Actor Object Reference") (OtherComp :type "PrimitiveComponent Object Reference") (bSelfMoved :type Boolean) (HitLocation :type "Vector Structure") (HitNormal :type "Vector Structure") (NormalImpulse :type "Vector Structure") (Hit :type "HitResult Structure (by ref)"))
  (bind _returnvalue (`GameplayStatics.GetPlayerCharacter` 0))
  (bind _returnvalue_2 (`GameplayStatics.GetPlayerCharacter` 0))
  (bind (_bblockinghit _binitialoverlap _time _distance _location _impactpoint _normal _impactnormal) (`GameplayStatics.BreakHitResult` Hit))
  (bind _returnvalue_3 (`self.K2_GetActorLocation`))
  (bind _returnvalue_4 (`self.K2_GetActorLocation` _returnvalue_2))
  (bind _capsulecomponent (`Character.CapsuleComponent` _returnvalue))
  (bind _returnvalue_5 (- _returnvalue_4 _returnvalue_3))
  (if (`self.bFalling`)
    _
    (elif (== _returnvalue_2 Other)
      (if (> (`KismetMathLibrary.Dot_VectorVector` _impactnormal (`self.GetActorForwardVector` _returnvalue_2)) 0.9)
        (bind _output_get (set `self.Pushable Direction` _impactnormal))
        (if (< (`KismetMathLibrary.VSize` (- _returnvalue_5 (* (`KismetMathLibrary.Dot_VectorVector` _returnvalue_5 _output_get) _output_get))) 100.0)
          (bind _result (`self.Can Push`))
          (if (!= _result 2)
            (`self.K2_SetActorRotation` _returnvalue_2 (`KismetMathLibrary.FindLookAtRotation` _returnvalue_4 (+ _returnvalue_3 (* _impactnormal 1000.0))) false)
            (`CharacterMovementComponent.DisableMovement` (`Character.CharacterMovement` _returnvalue))
            (`KismetSystemLibrary.MoveComponentTo` _capsulecomponent (+ (`SceneComponent.K2_GetComponentLocation` _capsulecomponent) (* (`self.GetActorForwardVector` _returnvalue) -45.0)) (`SceneComponent.K2_GetComponentRotation` _capsulecomponent))
            (`self.K2_AttachToActor` (`GameplayStatics.GetPlayerCharacter` 0) self "None" "KeepWorld" "KeepWorld" "KeepWorld" true)
            (`self.Push`)
            (else
              (`KismetSystemLibrary.PrintString` "cannot push"))))))))

(event `Push`
  (set `self.Current Location` (`self.K2_GetActorLocation`))
  (bind (_direction _position) (`Timeline|MoveBlock` :!via `PlayFromStart`)
    (:`Update`
      (`self.K2_SetActorRelativeLocation` (+ (`self.Current Location`) (* _position (`self.Pushable Direction`) (`self.Travel Distance`)))))
    (:`Finished`
      (if (`PlayerController.IsInputKeyDown` (`GameplayStatics.GetPlayerController` 0) "W")
        (bind _result (`self.Can Push`))
        (if (== _result 0)
          (`self.Push`)
          (else
            (`self.StopPushing`)))
        (else
          (`self.StopPushing`))))))

(event `StopPushing`
  (bind _returnvalue (`GameplayStatics.GetPlayerCharacter` 0))
  (`CharacterMovementComponent.SetMovementMode` (`Character.CharacterMovement` _returnvalue) "MOVE_Walking" 0)
  (`self.K2_DetachFromActor` _returnvalue "KeepWorld" "KeepWorld" "KeepWorld")
  (`|PlayMontage` (`Character.Mesh` (`GameplayStatics.GetPlayerCharacter` 0)) "/Game/Characters/Push/AM_PushMongtage.AM_PushMongtage" 2.0 0.0 "End"))

(event `self.Box.OnComponentBeginOverlap`
  (params (OverlappedComponent :type "PrimitiveComponent Object Reference") (OtherActor :type "Actor Object Reference") (OtherComp :type "PrimitiveComponent Object Reference") (OtherBodyIndex :type Integer) (bFromSweep :type Boolean) (SweepResult :type "HitResult Structure (by ref)"))
  (if (`self.bFalling`)
    _
    (elif (== OtherActor (`GameplayStatics.GetPlayerCharacter` 0))
      (`PrimitiveComponent.SetSimulatePhysics` (`self.Sphere`) false))))

(event `self.Box.OnComponentEndOverlap`
  (params (OverlappedComponent :type "PrimitiveComponent Object Reference") (OtherActor :type "Actor Object Reference") (OtherComp :type "PrimitiveComponent Object Reference") (OtherBodyIndex :type Integer))
  (if (== OtherActor (`GameplayStatics.GetPlayerCharacter` 0))
    (`PrimitiveComponent.SetSimulatePhysics` (`self.Sphere`) true)))

(event `self.ReceiveTick`
  (params (DeltaSeconds :type "Float (single-precision)"))
  (bind _returnvalue (`self.K2_GetActorLocation`))
  (bind _sphere (`self.Sphere`))
  (bind (_returnvalue_origin _returnvalue_boxextent) (`KismetMathLibrary.BreakBoxSphereBounds` (`StaticMesh.GetBounds` (`StaticMeshComponent.StaticMesh` _sphere))))
  (if (`self.bFalling`)
    (bind (_outhit _returnvalue_2) (`KismetSystemLibrary.BoxTraceSingle` _returnvalue (+ (+ _returnvalue (0.0 0.0 50.0)) (* (0.0 0.0 -1.0) (`self.Travel Distance`))) (`KismetMathLibrary.MakeVector` (.x (* _returnvalue_boxextent (`SceneComponent.RelativeScale3D` _sphere))) (.y (* _returnvalue_boxextent (`SceneComponent.RelativeScale3D` _sphere))) (* (.z (* _returnvalue_boxextent (`SceneComponent.RelativeScale3D` _sphere))) 0.2)) (struct) "TraceTypeQuery2" false (`|MakeArray` (`GameplayStatics.GetPlayerCharacter` 0)) "Persistent" true (struct :`R` 1.0 :`G` 1.0 :`B` 1.0 :`A` 1.0) (struct :`R` 1.0 :`G` 0.638993 :`A` 1.0))) ; 2. 절벽 박스로 체크
    (if _returnvalue_2
      (set `self.bFalling` false))))

(fn `Can Push`
  (returns (Result :type Integer))
  (bind _returnvalue (`self.K2_GetActorLocation`))
  (bind _sphere (`self.Sphere`))
  (bind _array (`|MakeArray` (`GameplayStatics.GetPlayerCharacter` 0)))
  (bind _returnvalue_2 (+ _returnvalue (0.0 0.0 50.0)))
  (bind (_returnvalue_origin _returnvalue_boxextent) (`KismetMathLibrary.BreakBoxSphereBounds` (`StaticMesh.GetBounds` (`StaticMeshComponent.StaticMesh` _sphere))))
  (bind _returnvalue_3 (* _returnvalue_boxextent (`SceneComponent.RelativeScale3D` _sphere)))
  (bind (_outhit _returnvalue_4) (`KismetSystemLibrary.BoxTraceSingle` _returnvalue_2 (+ _returnvalue_2 (* (`self.Pushable Direction`) (`self.Travel Distance`))) (* _returnvalue_3 0.9) (struct) "TraceTypeQuery2" false _array "ForDuration" true (struct :`A` 1.0) (struct :`G` 1.0 :`B` 0.940764 :`A` 1.0))) ; 1. 박스 앞 충돌 물체 확인
  (if (not _returnvalue_4)
    (bind (_outhit_2 _returnvalue_5) (`KismetSystemLibrary.BoxTraceSingle` _returnvalue (+ _returnvalue_2 (* (0.0 0.0 -1.0) (`self.Travel Distance`))) (`KismetMathLibrary.MakeVector` (.x _returnvalue_3) (.y _returnvalue_3) (* (.z _returnvalue_3) 0.2)) (struct) "TraceTypeQuery2" false _array "Persistent" true (struct :`R` 1.0 :`G` 1.0 :`B` 1.0 :`A` 1.0) (struct :`R` 1.0 :`G` 0.638993 :`A` 1.0))) ; 2. 절벽 박스로 체크
    (if _returnvalue_5
      (return 0)
      (else
        (set `self.bFalling` true)
        (`self.StopPushing`)
        (`PrimitiveComponent.SetSimulatePhysics` (`self.Sphere`) true)
        (return 1)))
    (else
      (`KismetSystemLibrary.PrintString` (`KismetSystemLibrary.GetDisplayName` (`.HitActor` (`GameplayStatics.BreakHitResult` _outhit))))
      (return 2))))

(fn `UserConstructionScript`)