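; BP_IceBlock is a reusable ice block actor that appears at the player character's horizontal position at a given height.
; CreateIceBlock enables collision, shows and moves the mesh, then deactivates it after a long delay.
; Deactivation and ResetIceBlock hide the mesh, disable collision and fire OnIceDestroyed rather than destroying the actor.
; A looping timer for ResetIceBlock exists but is unconnected.
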(event `self.ReceiveBeginPlay`)

(event `ResetIceBlock`
  (`self.OnIceDestroyed` self)
  (`PrimitiveComponent.SetCollisionEnabled` (`self.Ice`) "NoCollision")
  (`SceneComponent.SetVisibility` (`self.Ice`) false false))

(event `Create IceBlock`
  (params (Z :type "Float (double-precision)"))
  (bind (_returnvalue_x _returnvalue_y) (`KismetMathLibrary.BreakVector` (`SceneComponent.K2_GetComponentLocation` (`Character.Mesh` (`GameplayStatics.GetPlayerCharacter` 0)))))
  (`PrimitiveComponent.SetCollisionEnabled` (`self.Ice`) "QueryAndPhysics")
  (`SceneComponent.SetVisibility` (`self.Ice`) true false)
  (`self.K2_SetActorRotation` (struct))
  (`SceneComponent.K2_SetWorldLocation` (`self.Ice`) (`KismetMathLibrary.MakeVector` _returnvalue_x _returnvalue_y Z) false false)
  (`KismetSystemLibrary.Delay` 80.0)
  (`self.Deactive IceBlock`))

(event `Deactive IceBlock`
  (`PrimitiveComponent.SetCollisionEnabled` (`self.Ice`) "NoCollision")
  (`SceneComponent.SetVisibility` (`self.Ice`) false false)
  (`self.OnIceDestroyed` self))

(fn `UserConstructionScript`)