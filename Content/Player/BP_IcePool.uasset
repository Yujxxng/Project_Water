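; BP_IcePool is an object pool that pre-spawns BP_IceBlock actors for its owner.
; On BeginPlay it spawns AmountOfIce blocks at the owner's location, hides their mesh, disables collision, attaches them and stores them in IcePool.
; Each block's OnIceDestroyed event fires ReturnToPool, which moves it back to the owner and reattaches it.
; Pressing F calls DeactiveIceBlock on IcePool in a loop over AmountOfIce.
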(event `self.ReceiveBeginPlay`
  (for _ (range (+ (`self.AmountOfIce`) 1))
    (bind _returnvalue (`|SpawnActorFromClass` "/Game/Player/BP_IceBlock.BP_IceBlock_C" (`KismetMathLibrary.MakeTransform` (`Actor.K2_GetActorLocation` (`self.GetOwner`))) "Undefined" "MultiplyWithRoot" null null))
    (bind _ice (`/Game/Player/BP_IceBlock.Ice` _returnvalue))
    (`SceneComponent.SetVisibility` _ice false false)
    (`PrimitiveComponent.SetCollisionEnabled` _ice "NoCollision")
    (`Actor.K2_AttachToActor` _returnvalue (`self.GetOwner`) "None" "KeepWorld" "KeepWorld" "KeepWorld" true)
    (add `/Game/Player/BP_IceBlock.OnIceDestroyed` _returnvalue (delegate `ReturnToPool`))
    (`KismetArrayLibrary.Array_Add` (`self.IcePool`) _returnvalue)))

(event `ReturnToPool`
  (params (Ice :type "/Game/Player/BP_IceBlock Object Reference"))
  (bind _returnvalue (`self.GetOwner`))
  (`Actor.K2_SetActorLocation` Ice (`Actor.K2_GetActorLocation` _returnvalue) false false)
  (`Actor.K2_AttachToActor` Ice _returnvalue "None" "KeepWorld" "KeepWorld" "KeepWorld" true))

(event `Key|F`
  (params (Key :type "Key Structure"))
  (:`Pressed`
    (for _ (range (+ (`self.AmountOfIce`) 1))
      (`/Game/Player/BP_IceBlock.Deactive IceBlock` (`self.IcePool`)))))