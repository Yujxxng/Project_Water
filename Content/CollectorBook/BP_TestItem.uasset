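; Collectible item actor for the collector book, loading its data and mesh from the DT_ItemTable row named after the current level.
; On BeginPlay it checks WaterGameInstance and hides and disables collision if already collected, binding OnGetItem only in that case.
; Overlapping ShowWidgetArea toggles a widget.
; Interact destroys the actor, marks it collected, updates GM_WaterMode's collector and calls OnGetItemEvent with the ID.
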(event `self.ReceiveBeginPlay`
  (bind _returnvalue (`GameplayStatics.GetCurrentLevelName` true))
  (set `self.LevelName` _returnvalue)
  (`self.SetItem`)
  (bind _aswater_game_instance (cast `WaterGameInstance` (`GameplayStatics.GetGameInstance`)))
  (bind _returnvalue_2 (`WaterGameInstance.IsItemCollected` _aswater_game_instance (`self.ID`)))
  (bind _output_get (set `self.IsCollected` _returnvalue_2))
  (`SceneComponent.SetVisibility` (`self.StaticMesh`) (not _output_get) false)
  (if _output_get
    (`PrimitiveComponent.SetCollisionEnabled` (`self.CanInteratArea`) "NoCollision")
    (`PrimitiveComponent.SetCollisionEnabled` (`self.StaticMesh`) "NoCollision")
    (`PrimitiveComponent.SetCollisionEnabled` (`self.ShowWidgetArea`) "NoCollision")
    (add `self.OnGetItem` (delegate `OnGetItem_Event`))))

(event `OnGetItem_Event` :!signature `self.OnGetItem`
  (params (itemID :type String))
  (bind _asgm_water_mode (cast `/Game/GameMode/GM_WaterMode` (`GameplayStatics.GetGameMode`)))
  (`/Game/CollectorBook/WB_CollectorBook.UpdateCollector` (`/Game/GameMode/GM_WaterMode.CollectorBook` _asgm_water_mode) itemID))

(event `/Game/Actor/InteractActors/BPI_Interact.Interact`
  (bind _id (`self.ID`))
  (`self.K2_DestroyActor`)
  (set `self.IsCollected` true)
  (bind _asgm_water_mode (cast `/Game/GameMode/GM_WaterMode` (`GameplayStatics.GetGameMode`)))
  (`WaterGameMode.UpdateCollector` _asgm_water_mode _id)
  (`self.OnGetItem_Event` _id))

(event `self.ShowWidgetArea.OnComponentBeginOverlap`
  (params (OverlappedComponent :type "PrimitiveComponent Object Reference") (OtherActor :type "Actor Object Reference") (OtherComp :type "PrimitiveComponent Object Reference") (OtherBodyIndex :type Integer) (bFromSweep :type Boolean) (SweepResult :type "HitResult Structure (by ref)"))
  (`SceneComponent.SetVisibility` (`self.Widget`) true false))

(event `self.ShowWidgetArea.OnComponentEndOverlap`
  (params (OverlappedComponent :type "PrimitiveComponent Object Reference") (OtherActor :type "Actor Object Reference") (OtherComp :type "PrimitiveComponent Object Reference") (OtherBodyIndex :type Integer))
  (`SceneComponent.SetVisibility` (`self.Widget`) false false))

(fn `Set Data`
  (params (row :type "ItemTableRow Structure"))
  (`|ExecutionSequence`
    (:`then_0`
      (set `self.ID` row_ID))
    (:`then_1`
      (set `self.Name` row_Name))
    (:`then_2`
      (set `self.Detail` row_Detail))
    (:`then_3`
      (set `self.IsCollected` row_IsCollected))
    (:`then_4`
      (set `self.Textures` row_Textures))
    (:`then_5`
      (bind _output_get (set `self.Mesh` row_Mesh))
      (`StaticMeshComponent.SetStaticMesh` (`self.StaticMesh`) _output_get))))

(fn `SetItem`
  (bind _outrownames (`DataTableFunctionLibrary.GetDataTableRowNames` "/Game/CollectorBook/DT_ItemTable.DT_ItemTable"))
  (for _array_element _outrownames
    (if (== _array_element (`self.LevelName`))
      (bind _returnvalue (`|GetDataTableRow` "/Game/CollectorBook/DT_ItemTable.DT_ItemTable" _array_element)
        (:`then`
          (`self.Set Data` (make `ItemTableRow` (break `ItemTableRow` _returnvalue) (`.Name` (break `ItemTableRow` _returnvalue)) (`.Detail` (break `ItemTableRow` _returnvalue)) (`.IsCollected` (break `ItemTableRow` _returnvalue)) (`.Textures` (break `ItemTableRow` _returnvalue)) (`.Mesh` (break `ItemTableRow` _returnvalue)))))
        (:`RowNotFound`
          (`KismetSystemLibrary.PrintString` "Not found Lelvel == RowName Data"))))))

(fn `UserConstructionScript`)